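; BP_Card_Player is the player actor in a card game prototype, holding health and showing it on a WBP_HealthBar widget component.
; AnyDamage passes the hit to a TakeDamage function and stores the returned health, destroying the actor when that value is not above zero.
; SetHealthBarWidget updates the bar percentage and current/max text at BeginPlay and after each non-lethal hit.
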(event `self.ReceiveBeginPlay`
  ;[1 1 1] Setup
  (`self.SetHealthBarWidget`))

(event `self.ReceiveAnyDamage`
  (params (Damage :type "Float (single-precision)") (DamageType :type "DamageType Object Reference") (InstigatedBy :type "Controller Object Reference") (DamageCauser :type "Actor Object Reference"))
  ;[1 1 1] Take Damage
  (bind _returnhealth (`/Game/ProtoCards/UICards/BPFL_Cards.TakeDamage` (`self.health`) Damage self))
  (if (> _returnhealth 0.0)
    (set `self.health` _returnhealth)
    (`self.SetHealthBarWidget`)
    (else
      (`self.K2_DestroyActor`))))

(fn `SetHealthBarWidget`
  (bind _maxhealth (`self.maxHealth`))
  (bind _aswbp_health_bar (cast `/Game/Systems/CardCombatSystem/CombatEnemy/Widgets/WBP_HealthBar` (`WidgetComponent.GetWidget` (`self.WidgetHealthBar`))))
  (`ProgressBar.SetPercent` (`/Game/Systems/CardCombatSystem/CombatEnemy/Widgets/WBP_HealthBar.HealthBar` _aswbp_health_bar) (/ (`self.health`) _maxhealth))
  (`TextBlock.SetText` (`/Game/Systems/CardCombatSystem/CombatEnemy/Widgets/WBP_HealthBar.healthTxt` _aswbp_health_bar) (`|FormatText` "{H}/{MH}" (`self.health`) _maxhealth)))

(fn `UserConstructionScript`)