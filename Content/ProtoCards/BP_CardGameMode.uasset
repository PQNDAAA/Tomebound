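; Card combat game mode that sets up the card HUD with mouse input, disables pawn input, gathers all enemies and starts turn-based combat.
; TurnCombat dispatches on the turn enum, and SwitchTurn flips it, clearing the controller's selected-enemy arrow when the player's turn ends.
; Enemy turns run BT_AI on a random enemy and immediately pass play back; player turns clear that enemy's blackboard turn flag.
; Direct enemy damage and feedback logic is left unwired.
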(event `self.ReceiveBeginPlay`
  (bind _returnvalue (`GameplayStatics.GetPlayerController` 0))
  (bind _returnvalue_2 (`|CreateWidget` "/Game/ProtoCards/UICards/W_CardHUD.W_CardHUD_C" null (`self.cardNumber`)))
  (`UserWidget.AddToViewport` _returnvalue_2 0)
  (`WidgetBlueprintLibrary.SetInputMode_GameAndUIEx` _returnvalue _returnvalue_2)
  (set `PlayerController.bShowMouseCursor` true _returnvalue)
  (`self.DisableInput` (`GameplayStatics.GetPlayerPawn` 0) (`GameplayStatics.GetPlayerController` 0))
  (`self.AddEnemies`)
  (`self.StartGame`))

(event `playerTurn`
  ;[1 1 1] Player Turn
  (`KismetSystemLibrary.PrintString` "Player Turn")
  (`BlackboardComponent.SetValueAsBool` (`AIBlueprintHelperLibrary.GetBlackboard` (`AIBlueprintHelperLibrary.GetAIController` (`self.randomEnemyRef`))) "enemyTurn?" false))

(event `TurnCombat`
  (switch `/Game/Systems/CardCombatSystem/CombatEnemy/Enumeration/E_Turn` (`self.enum_Turn`)
    (:`NewEnumerator0`
      (`self.playerTurn`))
    (:`NewEnumerator1`
      (`self.enemyTurn`))))

(event `StartGame`
  ;[1 1 1] StartGame
  (`self.TurnCombat`))

(event `enemyTurn`
  ;[1 1 1] Enemy Turn
  (`KismetSystemLibrary.PrintString` "Enemy Turn")
  (set `self.randomEnemyRef` (`KismetArrayLibrary.Array_Random` (`self.enemiesNumber`)))
  (bind _returnvalue (`AIController.RunBehaviorTree` (`AIBlueprintHelperLibrary.GetAIController` (`self.randomEnemyRef`)) "/Game/Systems/CardCombatSystem/CombatEnemy/AI/BT_AI.BT_AI"))
  (if _returnvalue
    (`self.SwitchTurn`)
    (`self.TurnCombat`)))

(fn `AddEnemies`
  (bind _outactors (`GameplayStatics.GetAllActorsOfClass` "/Game/Systems/CardCombatSystem/CombatEnemy/AI/BP_Enemy.BP_Enemy_C"))
  (for _array_element _outactors
    (`KismetArrayLibrary.Array_AddUnique` (`self.enemiesNumber`) _array_element)))

(fn `SwitchTurn`
  (bind _asbp_card_controller (cast `/Game/ProtoCards/BP_CardController` (`GameplayStatics.GetPlayerController` 0) :!pure true))
  (bind _enemyreference (`/Game/ProtoCards/BP_CardController.enemyReference` _asbp_card_controller))
  (if (`|EnumEquality` (`self.enum_Turn`) "NewEnumerator0")
    (set `self.enum_Turn` "NewEnumerator1")
    (`/Engine/EditorBlueprintResources/StandardMacros.IsValid` _enemyreference
      (:`Is Valid`
        (set `/Game/ProtoCards/BP_CardController.isClickedOnEnemy` false _asbp_card_controller)
        (`SceneComponent.SetHiddenInGame` (`/Game/Systems/CardCombatSystem/CombatEnemy/AI/BP_Enemy.selectArrow` _enemyreference) true false)))
    (else
      (set `self.enum_Turn` "NewEnumerator0"))))

(fn `UserConstructionScript`)