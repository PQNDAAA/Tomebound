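; BP_CardController handles mouse selection of a combat enemy in the card game prototype.
; A left click traces under the cursor and, during the first turn state of BP_CardGameMode, stores the hit BP_CombatEnemy and shows its selection arrow.
; Only one enemy is held at a time, and clicking that same enemy again clears the selection.
; Space bar is a debug key that applies damage to the stored enemy.
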(event `Key|LeftMouseButton`
  (params (Key :type "Key Structure"))
  (bind _enemyreference (`self.enemyReference`))
  (:`Pressed`
    (bind _asbp_combat_enemy (cast `/Game/Systems/CardCombatSystem/CombatEnemy/BP_CombatEnemy` (`.HitActor` (`GameplayStatics.BreakHitResult` (`self.GetHitResultUnderCursorByChannel` "TraceTypeQuery1")))))
    ;[1 1 1] Check the turn to select a enemy
    (bind _asbp_card_game_mode (cast `/Game/ProtoCards/BP_CardGameMode` (`GameplayStatics.GetGameMode`)))
    (if (`|EnumEquality` (`/Game/ProtoCards/BP_CardGameMode.enum_Turn` _asbp_card_game_mode) "NewEnumerator0")
      ;[1 1 1] Check when draw the arrow
      (if (not (`self.isClickedOnEnemy`))
        (bind _output_get (set `self.enemyReference` _asbp_combat_enemy))
        (set `self.isClickedOnEnemy` true)
        (`SceneComponent.SetHiddenInGame` (`/Game/Systems/CardCombatSystem/CombatEnemy/BP_CombatEnemy.selectArrow` _output_get) false false)
        (else
          (`/Engine/EditorBlueprintResources/StandardMacros.IsValid` _enemyreference
            (:`Is Valid`
              (if (== _asbp_combat_enemy (`self.enemyReference`))
                (set `self.isClickedOnEnemy` false)
                (`SceneComponent.SetHiddenInGame` (`/Game/Systems/CardCombatSystem/CombatEnemy/BP_CombatEnemy.selectArrow` _enemyreference) true false)
                (set `self.enemyReference` null)))))))))

(event `Key|SpaceBar`
  (params (Key :type "Key Structure"))
  ;[1 1 1] Debug deal damage
  (:`Pressed`
    (`GameplayStatics.ApplyDamage` (`self.enemyReference`) 2.0 null self)))

(fn `UserConstructionScript`)