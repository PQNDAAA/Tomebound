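; Scrolling outfield effect that paints Niagara particle footprints into a render target and builds a stack of shell planes.
; Construction registers the actor as the Niagara spawner's callback and adds vertically layered, collision-free, shadowless planes with custom depth and their own lighting channel.
; Each particle callback stamps position and scaled size into OutfieldRenderTarget with a rock brush material.
; Tick draws a scroll material into that target, which is cleared on BeginPlay.
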(event `self.ReceiveBeginPlay`
  (`KismetRenderingLibrary.ClearRenderTarget2D` (`self.OutfieldRenderTarget`))
  (bind _returnvalue (`KismetMaterialLibrary.CreateDynamicMaterialInstance` "/Game/3D/Rendering/Material/M_OutfieldRTRockBrush.M_OutfieldRTRockBrush"))
  (set `self.RockBrushMaterial` _returnvalue))

(event `self.ReceiveTick`
  (params (DeltaSeconds :type "Float (single-precision)"))
  (`KismetRenderingLibrary.DrawMaterialToRenderTarget` (`self.OutfieldRenderTarget`) "/Game/3D/Rendering/Material/M_OutfieldRTRock_Scroll.M_OutfieldRTRock_Scroll"))

(event `self.ReceiveParticleData`
  (params (Data :type "Array of BasicParticleData Structure (by ref)") (NiagaraSystem :type "NiagaraSystem Object Reference") (SimulationPositionOffset :type "Vector Structure (by ref)"))
  (for _array_element Data
    (bind (_position _size) (break `BasicParticleData` _array_element))
    (bind (_x _y) (`KismetMathLibrary.BreakVector3f` _position))
    (`MaterialInstanceDynamic.SetVectorParameterValue` (`self.RockBrushMaterial`) "ParticleData" (`KismetMathLibrary.MakeColor` _x _y (* _size (`self.RockBrushSize`))))
    (`KismetRenderingLibrary.DrawMaterialToRenderTarget` (`self.OutfieldRenderTarget`) (`self.RockBrushMaterial`))))

(fn `UserConstructionScript`
  (bind _shell_amount (`self.Shell Amount`))
  (`|ExecutionSequence`
    (:`then_0`
      (`NiagaraComponent.SetNiagaraVariableObject` (`self.NS_ScrollingMeshSpawner`) "User.BP_Callback" self))
    (:`then_1`
      (for _index (range (+ _shell_amount 1))
        (bind _returnvalue (`AddComponent|NODE_AddStaticMeshComponent-0` :`RelativeTransform` (`KismetMathLibrary.MakeTransform` (* (/ (`KismetMathLibrary.Conv_IntToDouble` _index) (`KismetMathLibrary.Conv_IntToDouble` _shell_amount)) (`KismetMathLibrary.Vector_Up`)) (struct) (`KismetMathLibrary.Conv_DoubleToVector` (`self.Plane Scale`)))))
        (`PrimitiveComponent.SetRenderCustomDepth` _returnvalue true)
        (`PrimitiveComponent.SetCustomDepthStencilValue` _returnvalue 5)
        (`PrimitiveComponent.SetLightingChannels` _returnvalue false true false)
        (`PrimitiveComponent.SetCollisionEnabled` _returnvalue "NoCollision")
        (`PrimitiveComponent.SetCastShadow` _returnvalue false)))))