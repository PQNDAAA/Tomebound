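; Actor component that scrolls its owning actor along the Y axis in a repeating loop.
; Each Tick it adds Speed times delta time to the owner's Y and wraps the result with a modulo over the LoopStart-to-LoopEnd span, offset from LoopEnd.
; X and Z carry over from the world location, but the result is written as relative location without sweep, so the two match only for unparented actors.
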(event `self.ReceiveTick`
  (params (DeltaSeconds :type "Float (single-precision)"))
  (bind _returnvalue (`self.GetOwner`))
  (`Actor.K2_SetActorRelativeLocation` _returnvalue (`KismetMathLibrary.MakeVector` (.x (`Actor.K2_GetActorLocation` _returnvalue)) (+ (`self.Loop End`) (mod (- (+ (.y (`Actor.K2_GetActorLocation` _returnvalue)) (* DeltaSeconds (`self.Speed`))) (`self.Loop End`)) (- (`self.Loop Start`) (`self.Loop End`))) 0.0) (.z (`Actor.K2_GetActorLocation` _returnvalue))) false false))