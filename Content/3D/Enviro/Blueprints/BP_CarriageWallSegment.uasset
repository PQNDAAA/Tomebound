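; Modular train carriage wall segment, configured entirely in the Construction Script with no active runtime logic.
; Variant swaps the inside, outside and glass meshes, with the third variant removing the glass.
; Toggles strip the optional joint, railing and rolling curtain components when unused.
; CurtainPos height places the curtain pull, and its clamped drop scales the stretch mesh and lerps the roll's thickness between rolled and unrolled.
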(fn `UserConstructionScript`
  (bind _curtainminpull (`self.curtainMinPull`))
  (bind _z (.z (`self.curtainPos`)))
  (bind (_x _y) (`KismetMathLibrary.BreakVector3f` (`SceneComponent.RelativeLocation` (`self.SM_CurtainRollingPull`))))
  (bind _returnvalue (`KismetMathLibrary.FMax` (`KismetMathLibrary.FMin` (- (.z (`SceneComponent.RelativeLocation` (`self.SM_CurtainRollingStretch`))) _z) (`self.curtainMaxPull`)) (`self.curtainMinPull`)))
  (bind _returnvalue_2 (`KismetMathLibrary.Lerp` (`self.curtainRolledScale`) (`self.curtainUnrolledScale`) (/ (- _returnvalue _curtainminpull) (- (`self.curtainMaxPull`) _curtainminpull))))
  (`|ExecutionSequence`
    (:`then_0`
      (switch `int` (`self.Variant`)
        (:`2`
          (`StaticMeshComponent.SetStaticMesh` (`self.SM_InsideWall`) "/Game/3D/Enviro/Meshes/SM_CarriageWall_02.SM_CarriageWall_02")
          (`StaticMeshComponent.SetStaticMesh` (`self.SM_CarriageWall_01_Outside`) "/Game/3D/Enviro/Meshes/SM_CarriageWall_02_Outside.SM_CarriageWall_02_Outside")
          (`StaticMeshComponent.SetStaticMesh` (`self.SM_CarriageWall_01_Glass`) "/Game/3D/Enviro/Meshes/SM_CarriageWall_02_Glass.SM_CarriageWall_02_Glass"))
        (:`3`
          (`StaticMeshComponent.SetStaticMesh` (`self.SM_InsideWall`) "/Game/3D/Enviro/Meshes/SM_CarriageWall_03.SM_CarriageWall_03")
          (`StaticMeshComponent.SetStaticMesh` (`self.SM_CarriageWall_01_Outside`) "/Game/3D/Enviro/Meshes/SM_CarriageWall_03_Outside.SM_CarriageWall_03_Outside")
          (`ActorComponent.K2_DestroyComponent` (`self.SM_CarriageWall_01_Glass`)))))
    (:`then_1`
      (if (not (`self.Add joint`))
        (`ActorComponent.K2_DestroyComponent` (`self.SM_CarriageWallJoint_01`))))
    (:`then_2`
      (if (not (`self.addRailing`))
        (`ActorComponent.K2_DestroyComponent` (`self.SM_CarriageWallRailing_01`))))
    (:`then_4`
      (if (`self.addRollingCurtain`)
        (`SceneComponent.K2_SetRelativeLocation` (`self.SM_CurtainRollingPull`) (`KismetMathLibrary.MakeVector` _x _y _z) false false)
        (`SceneComponent.SetRelativeScale3D` (`self.SM_CurtainRollingStretch`) (`KismetMathLibrary.MakeVector` 1.0 1.0 (/ _returnvalue 5.0)))
        (`SceneComponent.SetRelativeScale3D` (`self.SM_CurtainRollingRoll`) (`KismetMathLibrary.MakeVector` 1.0 _returnvalue_2 _returnvalue_2))
        (else
          (`ActorComponent.K2_DestroyComponent` (`self.SM_CurtainRollingFixed`))
          (`ActorComponent.K2_DestroyComponent` (`self.SM_CurtainRollingStretch`))
          (`ActorComponent.K2_DestroyComponent` (`self.SM_CurtainRollingPull`))
          (`ActorComponent.K2_DestroyComponent` (`self.SM_CurtainRollingRoll`)))))))