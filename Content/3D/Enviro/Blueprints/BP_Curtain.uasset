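; BP_Curtain is a configurable environment prop that assembles a curtain from five static mesh parts.
; The construction script assigns meshes from variables to left and right curtains, two ropes and a top piece.
; An optional MirrorTopCurtain flag flips the top piece by setting a negative X scale.
; The event graph holds only disabled stub events, so it has no runtime logic.
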(fn `UserConstructionScript`
  (`StaticMeshComponent.SetStaticMesh` (`self.SM_CurtainLong_01`) (`self.Left Curtain`))
  (`StaticMeshComponent.SetStaticMesh` (`self.SM_CurtainLong_02`) (`self.Right Curtain`))
  (`StaticMeshComponent.SetStaticMesh` (`self.SM_CurtainRope_01`) (`self.Left Rope`))
  (`StaticMeshComponent.SetStaticMesh` (`self.SM_CurtainRope_02`) (`self.Right Rope`))
  (`StaticMeshComponent.SetStaticMesh` (`self.SM_CurtainTop_01`) (`self.Top Curtain`))
  (if (`self.Mirror Top Curtain`)
    (`SceneComponent.SetRelativeScale3D` (`self.SM_CurtainTop_01`) (`KismetMathLibrary.MakeVector` -1.0 1.0 1.0))))