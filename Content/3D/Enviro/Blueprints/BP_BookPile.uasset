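; Procedural environment prop that builds a vertical pile of books as mesh instances on the Books component.
; The construction script derives the book count from the Z position of PileHeight and the average book thickness.
; It rolls a thickness per book, accumulates these into stacked offsets, then adds instances with random yaw and width/depth scale.
; Randomness is unseeded, so each reconstruction reshuffles the pile, and its actual height only approximates PileHeight.
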(fn `UserConstructionScript`
  (bind _returnvalue (`KismetMathLibrary.RandomFloatInRange` 0.8 1.2))
  (`|ExecutionSequence`
    (:`then_0`
      (set `self.Book Amount` (`KismetMathLibrary.FTrunc` (/ (.z (.location (`self.Pile Height`))) (* (+ (`self.Min Relative Book Thickness`) (`self.Max Relative Book Thickness`)) (`self.Book Thickness`) 0.5)))))
    (:`then_1`
      (set `InstancedStaticMeshComponent.InstancingRandomSeed` (`KismetMathLibrary.RandomIntegerInRange` 1 150000) (`self.Books`)))
    (:`then_2`
      (`KismetArrayLibrary.Array_Clear` (`self.thicknesses`))
      (for _ (range (`self.Book Amount`))
        (`KismetArrayLibrary.Array_Add` (`self.thicknesses`) (`KismetMathLibrary.RandomFloatInRange` (`self.Min Relative Book Thickness`) (`self.Max Relative Book Thickness`)))))
    (:`then_3`
      (if (> (`self.Book Amount`) 0)
        (`KismetArrayLibrary.Array_Clear` (`self.locations`))
        (`KismetArrayLibrary.Array_Add` (`self.locations`))
        (for _index (range (+ (- (`self.Book Amount`) 2) 1))
          (`KismetArrayLibrary.Array_Add` (`self.locations`) (+ (`|GetArrayItem` (`self.locations`) (- _index 0)) (* (`|GetArrayItem` (`self.thicknesses`) _index) (`self.Book Thickness`)))))))
    (:`then_4`
      (for (_array_element _array_index) (`self.locations`)
        (`InstancedStaticMeshComponent.AddInstance` (`self.Books`) (`KismetMathLibrary.MakeTransform` (`KismetMathLibrary.MakeVector` 0.0 0.0 _array_element) (`KismetMathLibrary.MakeRotator` 0.0 0.0 (`KismetMathLibrary.RandomFloatInRange` 0.0 360.0)) (`KismetMathLibrary.MakeVector` _returnvalue _returnvalue (`|GetArrayItem` (`self.thicknesses`) _array_index))) false)))))