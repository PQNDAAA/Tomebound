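; Modular train carriage end-wall segment with a selectable Variant, built from wall, wall glass, door and door glass mesh components.
; The construction script keeps the default end wall with door unless Variant is 1 or 2.
; Those variants destroy the door and door glass components and swap the wall and glass meshes to the matching doorless end-wall meshes.
; The event graph holds no logic.
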(fn `UserConstructionScript`
  (switch `int` (`self.Variant`)
    (:`1`
      (`ActorComponent.K2_DestroyComponent` (`self.SM_CarriageWallEndDoor_01_DoorGlass`))
      (`ActorComponent.K2_DestroyComponent` (`self.SM_CarriageWallEndDoor_01_Door`))
      (`StaticMeshComponent.SetStaticMesh` (`self.SM_CarriageWallEndDoor_01`) "/Game/3D/Enviro/Meshes/SM_CarriageWallEnd_01.SM_CarriageWallEnd_01")
      (`StaticMeshComponent.SetStaticMesh` (`self.SM_CarriageWallEndDoor_01_Glass`) "/Game/3D/Enviro/Meshes/SM_CarriageWallEnd_01_Glass.SM_CarriageWallEnd_01_Glass"))
    (:`2`
      (`ActorComponent.K2_DestroyComponent` (`self.SM_CarriageWallEndDoor_01_DoorGlass`))
      (`ActorComponent.K2_DestroyComponent` (`self.SM_CarriageWallEndDoor_01_Door`))
      (`StaticMeshComponent.SetStaticMesh` (`self.SM_CarriageWallEndDoor_01`) "/Game/3D/Enviro/Meshes/SM_CarriageWallEnd_02.SM_CarriageWallEnd_02")
      (`StaticMeshComponent.SetStaticMesh` (`self.SM_CarriageWallEndDoor_01_Glass`) "/Game/3D/Enviro/Meshes/SM_CarriageWallEnd_02_Glass.SM_CarriageWallEnd_02_Glass"))))