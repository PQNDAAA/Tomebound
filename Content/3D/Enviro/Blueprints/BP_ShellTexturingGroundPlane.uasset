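; BP_ShellTexturingGroundPlane builds a shell-textured outfield ground from stacked static mesh planes.
; The construction script adds scaled plane components in a loop, spacing them evenly upward from GroundLevel using ShellAmount and ShellsThickness.
; Every layer shares MI_Outfield with no per-shell parameters, writes custom depth stencil, uses lighting channels 1 and 2, and disables collision and shadows.
; The event graph has no runtime logic.
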(fn `UserConstructionScript`
  (bind _shell_amount (`self.Shell Amount`))
  (for _index (range (+ _shell_amount 1))
    (bind _returnvalue (`AddComponent|NODE_AddStaticMeshComponent-0` :`RelativeTransform` (`KismetMathLibrary.MakeTransform` (+ (* _index (/ (`self.Shells Thickness`) _shell_amount) (`KismetMathLibrary.Vector_Up`)) (* (`KismetMathLibrary.Vector_Up`) (`self.Ground Level`))) (struct) (`KismetMathLibrary.Conv_DoubleToVector` (`self.Plane Scale`)))))
    (`PrimitiveComponent.SetRenderCustomDepth` _returnvalue true)
    (`PrimitiveComponent.SetCustomDepthStencilValue` _returnvalue 5)
    (`PrimitiveComponent.SetMaterial` _returnvalue 0 "/Game/3D/Enviro/Materials/MI_Outfield.MI_Outfield")
    (`PrimitiveComponent.SetLightingChannels` _returnvalue false true true)
    (`PrimitiveComponent.SetCollisionEnabled` _returnvalue "NoCollision")
    (`PrimitiveComponent.SetCastShadow` _returnvalue false)))