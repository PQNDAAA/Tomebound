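; BP_Object is an interactable world object that opens a dialog widget with its text when left-clicked while something overlaps its Box.
; Overlap toggles input and a gate; the click requires a cursor trace hit on an "ObjectActor"-tagged actor and no active dialog, then disables player pawn input.
; A looping timer replays a timeline that draws a shrinking debug circle around the Cube until the dialog block is hidden, then clears the reference.
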(event `Key|LeftMouseButton`
  (params (Key :type "Key Structure"))
  (:`Pressed`
    (`/Engine/EditorBlueprintResources/StandardMacros.Gate` true :!label _label
      (:`Exit`
        (if (and (`self.ActorHasTag` (`.HitActor` (`GameplayStatics.BreakHitResult` (`PlayerController.GetHitResultUnderCursorByChannel` (`GameplayStatics.GetPlayerController` 0) "TraceTypeQuery1" true))) "ObjectActor") (not (`KismetSystemLibrary.IsValid` (`self.WBP_ObjectDialogReference`))))
          (`self.DisableInput` (`GameplayStatics.GetPlayerPawn` 0) (`GameplayStatics.GetPlayerController` 0))
          (bind _returnvalue (`|CreateWidget` "/Game/Widgets/WBP_ObjectDialog.WBP_ObjectDialog_C"))
          (bind _output_get (set `self.WBP_ObjectDialogReference` _returnvalue))
          (`UserWidget.AddToViewport` _output_get 0)
          (`/Game/Utilities/Librairies/BFL_Main.SetDialogBlockOnWidget` (`/Game/Widgets/WBP_ObjectDialog.DialogBlock` (`self.WBP_ObjectDialogReference`)) (`self.dialogText`))
          (bind _returnvalue_2 (`KismetSystemLibrary.K2_SetTimerDelegate` (delegate `DrawCircle`) 2.0 true))
          (set `self.timerHandleDrawCircle` _returnvalue_2))))))

(event `self.Box.OnComponentBeginOverlap`
  (params (OverlappedComponent :type "PrimitiveComponent Object Reference") (OtherActor :type "Actor Object Reference") (OtherComp :type "PrimitiveComponent Object Reference") (OtherBodyIndex :type Integer) (bFromSweep :type Boolean) (SweepResult :type "HitResult Structure (by ref)"))
  (`self.EnableInput` (`GameplayStatics.GetPlayerController` 0))
  (goto _label :!via `Open`))

(event `self.Box.OnComponentEndOverlap`
  (params (OverlappedComponent :type "PrimitiveComponent Object Reference") (OtherActor :type "Actor Object Reference") (OtherComp :type "PrimitiveComponent Object Reference") (OtherBodyIndex :type Integer))
  (`self.DisableInput` (`GameplayStatics.GetPlayerController` 0))
  (goto _label :!via `Close`))

(event `DrawCircle`
  (bind (_returnvalue_x _returnvalue_y) (`KismetMathLibrary.BreakVector` (`SceneComponent.K2_GetComponentLocation` (`self.Cube`))))
  (if (`Widget.IsVisible` (`/Game/Widgets/WBP_ObjectDialog.DialogBlock` (`self.WBP_ObjectDialogReference`)))
    (bind (_direction _tracksize) (`Timeline|Timeline` :!via `PlayFromStart`)
      (:`Update`
        (`KismetSystemLibrary.DrawDebugCircle` (`KismetMathLibrary.MakeVector` _returnvalue_x _returnvalue_y) (`KismetMathLibrary.Lerp` 150.0 0.0 _tracksize) 40 (struct :`R` 0.042341 :`G` 0.739583 :`A` 1.0) 0.1 6.0 (1.0 0.0 0.0) (0.0 1.0 0.0))))
    (else
      (`KismetSystemLibrary.K2_ClearAndInvalidateTimerHandle` (`self.timerHandleDrawCircle`))
      (set `self.WBP_ObjectDialogReference` null))))

(fn `UserConstructionScript`)