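; Player character for Tomebound with right-click movement, interaction, seating and an orbit camera.
; Clicks draw a shrinking debug circle, then navigate via SimpleMoveToLocation; a delayed velocity poll triggers the target's interaction and turns the capsule.
; Mouse wheel zoom drives spring arm pitch, while middle-drag applies limited yaw.
; Keys toggle pause, dialog, affinity, monologue and debug UI, with tutorial gates and mission updates; axis movement is disconnected.
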(event `self.ReceiveBeginPlay`
  (set `PlayerController.bShowMouseCursor` true (`GameplayStatics.GetPlayerController` 0))
  (`/Game/Utilities/GameInstance/GameInstance_Tomebound.AccessToViewportDebugChat` (`/Game/Utilities/Librairies/BFL_Main.GetGameInstanceTomebound`)))

(event `InputAxis|Move Forward/Backward`
  (params (AxisValue :type "Float (single-precision)")))

(event `InputAxis|Move Left/Right`
  (params (AxisValue :type "Float (single-precision)")))

(event `TranslationCharacterRotation`
  (params (Target :type "/Game/Systems/BP_ObjectBase Object Reference"))
  (bind _capsulecomponent (`self.CapsuleComponent`))
  (bind (_returnvalue_roll _returnvalue_pitch _returnvalue_yaw) (`KismetMathLibrary.BreakRotator` (`SceneComponent.K2_GetComponentRotation` (`/Game/Systems/BP_ObjectBase.Arrow` Target))))
  (bind (_returnvalue_roll_2 _returnvalue_pitch_2 _returnvalue_yaw_2) (`KismetMathLibrary.BreakRotator` (`SceneComponent.K2_GetComponentRotation` _capsulecomponent)))
  ;[1 1 1] Rotate Player to the Character Rotation
  (bind (_direction _tracksize) (`Timeline|Timeline_0` :!via `PlayFromStart`)
    (:`Update`
      (`SceneComponent.K2_SetWorldRotation` _capsulecomponent (`KismetMathLibrary.MakeRotator` _returnvalue_roll_2 _returnvalue_pitch_2 (`KismetMathLibrary.Lerp` _returnvalue_yaw _returnvalue_yaw_2 _tracksize)) false false))))

(event `Key|LeftMouseButton`
  (params (Key :type "Key Structure")))

(event `Key|RightMouseButton`
  (params (Key :type "Key Structure"))
  ;[1 1 1] ClickToMoveSystem
  (:`Pressed`
    (if (and (`self.IsCameraTutoCompl?`) (not (`self.isSitting?`)))
      (set `self.Location` (`.Location` (`GameplayStatics.BreakHitResult` (`PlayerController.GetHitResultUnderCursorByChannel` (`GameplayStatics.GetPlayerController` 0) "TraceTypeQuery1" true))))
      (`KismetSystemLibrary.K2_SetTimerDelegate` (delegate `DrawCircle`) 0.01))))

(event `CheckPath`
  (params (Target :type "/Game/Systems/BP_ObjectBase Object Reference"))
  ;[1 1 1] Check walking to intract with objects
  (`/Engine/EditorBlueprintResources/StandardMacros.IsValid` Target
    (:`Is Valid`
      (`KismetSystemLibrary.Delay` 0.2)
      (if (`KismetMathLibrary.NearlyEqual_FloatFloat` (`KismetMathLibrary.VSize` (`self.GetVelocity`)) 0.0 80.0)
        (`/Game/Systems/BP_ObjectBase.ObjectInteraction` Target)
        (`self.TranslationCharacterRotation` Target)
        (set `self.ObjectBaseRef` null)
        (`KismetSystemLibrary.PrintString` "PATH IS FINISHED" true true (struct :`R` 1.0 :`G` 0.028119 :`B` 0.311 :`A` 1.0))
        (else
          (`self.CheckPath` Target))))))

(event `DrawCircle`
  ;[1 1 1] ClickToMoveSystem
  (bind (_direction _tracksize) (`Timeline|Timeline` :!via `PlayFromStart`)
    (:`Update`
      (`KismetSystemLibrary.DrawDebugCircle` (`self.Location`) (`KismetMathLibrary.Lerp` 50.0 0.0 _tracksize) 40 (struct :`R` 0.630201 :`G` 1.0 :`B` 0.62 :`A` 1.0) 0.0 7.5 (1.0 0.0 0.0) (0.0 1.0 0.0)))
    (:`Finished`
      (bind (_returnvalue _object) (message `/Game/Systems/BPI_ObjectBase.isAnObject?` (`.HitActor` (`GameplayStatics.BreakHitResult` (`PlayerController.GetHitResultUnderCursorByChannel` (`GameplayStatics.GetPlayerController` 0) "TraceTypeQuery1" true)))))
      (if _returnvalue
        (set `/Game/Systems/BP_ObjectBase.startCollider` false _object)
        (bind _output_get (set `self.ObjectBaseRef` _object))
        (`AIBlueprintHelperLibrary.SimpleMoveToLocation` (`self.GetController`) (`SceneComponent.K2_GetComponentLocation` (`/Game/Systems/BP_ObjectBase.Sphere` _output_get)))
        (else
          (`AIBlueprintHelperLibrary.SimpleMoveToLocation` (`self.GetController`) (`self.Location`))))
      (`/Game/Utilities/Librairies/BFL_Main.PrintDebugChat` (`|FormatText` "MovePlayer" (`KismetStringLibrary.Conv_VectorToString` (`self.Location`))) "MovePlayer")
      (`self.CheckPath` (`self.ObjectBaseRef`)))))

(event `Key|I`
  (params (Key :type "Key Structure"))
  ;[1 0.1146 0.1146] Show Dialog UI
  (:`Pressed`
    (`/Engine/EditorBlueprintResources/StandardMacros.FlipFlop`
      (:`A`
        (bind _dialoghudreference (`self.DialogHUDReference`)
          (:`then`
            (`Widget.SetVisibility` _dialoghudreference "Visible"))
          (:`else`
            (bind _returnvalue (`|CreateWidget` "/Game/Widgets/WBP_Dialog.WBP_Dialog_C"))
            (bind _output_get (set `self.DialogHUDReference` _returnvalue))
            (`UserWidget.AddToViewport` _output_get 0))))
      (:`B`
        (`Widget.SetVisibility` _dialoghudreference "Hidden")))))

(event `InputAxisKey|MouseWheelAxis`
  (params (AxisValue :type "Float (single-precision)"))
  (bind _springarm (`self.SpringArm`))
  ;[1 1 1] Camera Zoom
  (set `self.springArmSmoothing` (`KismetMathLibrary.FClamp` (+ (* AxisValue -65.0) (`self.springArmSmoothing`)) (`self.CameraMinDistance`) (`self.CameraMaxDistance`)))
  (set `SpringArmComponent.TargetArmLength` (`KismetMathLibrary.FInterpTo` (`SpringArmComponent.TargetArmLength` _springarm) (`self.springArmSmoothing`) (`GameplayStatics.GetWorldDeltaSeconds`) 2.0) _springarm)
  (`self.SetCameraPitchFromZoom`))

(event `Key|MiddleMouseButton`
  (params (Key :type "Key Structure"))
  ;[1 1 1] Camera Yaw
  (:`Pressed`
    (set `self.CameraYawMousePressed` true)
    (bind _returnvalue (`WidgetLayoutLibrary.GetMousePositionOnViewport`))
    (set `self.CameraYawClickOrigin` _returnvalue))
  (:`Released`
    (set `self.CameraYawMousePressed` false)
    (bind _returnvalue_2 (`GameplayStatics.GetCurrentLevelName` true))
    (if (`KismetStringLibrary.EqualEqual_StrStr` _returnvalue_2 "LVL_Persistent_Tuto")
      (`/Engine/EditorBlueprintResources/StandardMacros.DoOnce` false
        (:`Completed`
          (`/Game/Player/GM_Tomebound.updateMission1` (`/Game/Systems/Tutorial/BPL_Tuto.cast GM_Tomebound`)))))))

(event `InputAction|OptionsMenu`
  (params (Key :type "Key Structure"))
  (bind _returnvalue (`GameplayStatics.GetPlayerController` 0))
  ;[1 1 1] Pause Menu
  (:`Pressed`
    (`|ExecutionSequence`
      (:`then_0`
        (bind _returnvalue_2 (`GameplayStatics.GetCurrentLevelName` true))
        (if (`KismetStringLibrary.EqualEqual_StrStr` _returnvalue_2 "LVL_MAINMENU")
          (set `self.PauseMenuAvailable?` false)
          (else
            (set `self.PauseMenuAvailable?` true))))
      (:`then_1`
        (`self.DisableInput` (`GameplayStatics.GetPlayerCharacter` 0) (`GameplayStatics.GetPlayerController` 0))
        (if (`self.PauseMenuAvailable?`)
          (if (`GameplayStatics.IsGamePaused`)
            (`GameplayStatics.SetGamePaused` false)
            (set `PlayerController.bShowMouseCursor` true _returnvalue)
            (`Widget.RemoveFromParent` (stale _returnvalue_3))
            (`self.EnableInput` (`GameplayStatics.GetPlayerCharacter` 0) (`GameplayStatics.GetPlayerController` 0))
            (else
              (`GameplayStatics.SetGamePaused` true)
              (set `PlayerController.bShowMouseCursor` true _returnvalue)
              (bind _returnvalue_3 (`|CreateWidget` "/Game/Main_Menu/UI/BP/Pause_Menu.Pause_Menu_C"))
              (`UserWidget.AddToViewport` _returnvalue_3 0))))))))

(event `self.ReceiveTick`
  (params (DeltaSeconds :type "Float (single-precision)"))
  ;[1 1 1] Camera Yaw
  (`self.SetCameraTargetYaw`))

(event `Key|V`
  (params (Key :type "Key Structure"))
  ;[1 1 1] Debug Chat Visibility
  (:`Pressed`
    (`/Engine/EditorBlueprintResources/StandardMacros.FlipFlop`
      (:`A`
        (`/Game/Utilities/Librairies/BFL_Main.VisibilityDebugChat` "Visible"))
      (:`B`
        (`/Game/Utilities/Librairies/BFL_Main.VisibilityDebugChat` "Hidden")))))

(event `InputAction|AffinityMenu`
  (params (Key :type "Key Structure"))
  (:`Pressed`
    (if (`self.IsAffinityTutoCompl?`)
      (`/Engine/EditorBlueprintResources/StandardMacros.FlipFlop`
        (:`A`
          (bind _affinitybarref (`self.AffinityBarRef`)
            (:`then`
              (`Widget.SetVisibility` _affinitybarref "Visible"))
            (:`else`
              (bind _returnvalue (`|CreateWidget` "/Game/Systems/AffinitySystem/Widgets/WBP_AffinityBarHUD.WBP_AffinityBarHUD_C"))
              (bind _output_get (set `self.AffinityBarRef` _returnvalue))
              (`UserWidget.AddToViewport` _output_get 0))))
        (:`B`
          (`Widget.SetVisibility` _returnvalue "Hidden")
          (`/Engine/EditorBlueprintResources/StandardMacros.DoOnce` false
            (:`Completed`
              (`/Game/Player/GM_Tomebound.updateMission4` (`/Game/Systems/Tutorial/BPL_Tuto.cast GM_Tomebound`))
              (bind _asgame_instance_tomebound (cast `/Game/Utilities/GameInstance/GameInstance_Tomebound` (`GameplayStatics.GetGameInstance`)))
              (set `/Game/Utilities/GameInstance/GameInstance_Tomebound.allTutoCompleted` true _asgame_instance_tomebound))))))))

(event `Key|C`
  (params (Key :type "Key Structure"))
  (:`Pressed`
    (`KismetSystemLibrary.Delay` 1.0)
    (`/Engine/EditorBlueprintResources/StandardMacros.FlipFlop`
      (:`A`
        (bind _affinitypanelref (`self.AffinityPanelRef`)
          (:`then`
            (`/Game/Widgets/WBP_AffinityPanel.PanelDown` _affinitypanelref))
          (:`else`
            (bind _returnvalue (`|CreateWidget` "/Game/Widgets/WBP_AffinityPanel.WBP_AffinityPanel_C"))
            (bind _output_get (set `self.AffinityPanelRef` _returnvalue))
            (`UserWidget.AddToViewport` _output_get 0))))
      (:`B`
        (`/Game/Widgets/WBP_AffinityPanel.PanelUp` (`self.AffinityPanelRef`))))))

(event `Key|Enter`
  (params (Key :type "Key Structure"))
  (:`Pressed`
    (`Widget.RemoveFromParent` (`self.Widget_Monologue`))))

(event `Key|K`
  (params (Key :type "Key Structure"))
  (:`Pressed`
    (bind _returnvalue (`|CreateWidget` "/Game/Systems/Characters/Widgets/WBP_Monologue.WBP_Monologue_C"))
    (bind _output_get (set `self.Widget_Monologue` _returnvalue))
    (`UserWidget.AddToViewport` _output_get 0)))

(event `Key|T`
  (params (Key :type "Key Structure"))
  (:`Pressed`
    (bind (_returnvalue _object) (message `/Game/Systems/BPI_ObjectBase.isAnObject?` (stale `self.CapsuleComponent.OnComponentBeginOverlap` OtherActor)))
    (bind (_asbp_seat_actor _bsuccess) (cast `/Game/Systems/SitSystem/BP_SeatActor` _object :!pure true))
    (if _bsuccess
      (`/Engine/EditorBlueprintResources/StandardMacros.Gate` true :!label _label
        (:`Exit`
          (`/Engine/EditorBlueprintResources/StandardMacros.FlipFlop`
            (:`A`
              (set `self.isSitting?` true)
              (bind _returnvalue_location (`KismetMathLibrary.BreakTransform` (`SceneComponent.K2_GetComponentToWorld` (`/Game/Systems/SitSystem/BP_SeatActor.targetPointSit` _asbp_seat_actor))))
              (bind (_relativerotation_roll _relativerotation_pitch _relativerotation_yaw) (`KismetMathLibrary.BreakRotator` (`SceneComponent.RelativeRotation` (`/Game/Systems/BP_ObjectBase.Arrow` _asbp_seat_actor))))
              (`SceneComponent.K2_SetWorldTransform` (`self.CapsuleComponent`) (`KismetMathLibrary.MakeTransform` _returnvalue_location (`KismetMathLibrary.MakeRotator` 0.0 0.0 (+ (* _relativerotation_yaw -1.0) (.yaw (.rotation (`self.GetTransform` _asbp_seat_actor)))))) false false))
            (:`B`
              (set `self.isSitting?` false))))))))

(event `self.CapsuleComponent.OnComponentBeginOverlap`
  (params (OverlappedComponent :type "PrimitiveComponent Object Reference") (OtherActor :type "Actor Object Reference") (OtherComp :type "PrimitiveComponent Object Reference") (OtherBodyIndex :type Integer) (bFromSweep :type Boolean) (SweepResult :type "HitResult Structure (by ref)"))
  (goto _label :!via `Open`))

(event `self.CapsuleComponent.OnComponentEndOverlap`
  (params (OverlappedComponent :type "PrimitiveComponent Object Reference") (OtherActor :type "Actor Object Reference") (OtherComp :type "PrimitiveComponent Object Reference") (OtherBodyIndex :type Integer))
  (goto _label :!via `Close`))

(fn `GetCameraYawOffset`
  (params (MouseVelocity :type "Vector2D Structure"))
  (returns (ReturnValue :type "Float (double-precision)"))
  (bind _returnvalue (* (`KismetMathLibrary.BreakVector2D` MouseVelocity) (`self.CameraYawSpeed`)))
  (if (`self.InvertYawControl`)
    (return _returnvalue)
    (else
      (return (* _returnvalue -1.0)))))

(fn `GetCameraZoomStep`
  (params (isZoomIn :type Boolean))
  (returns (ZoomStep :type "Float (double-precision)"))
  (return (`self.CameraZoomStep`)))

(fn `IsPlayer?`
  (returns (returnValue :type Boolean) (player :type "/Game/Player/BP_Player Object Reference"))
  (bind _returnvalue (`self.IsPlayerControlled`))
  (if _returnvalue
    (return _returnvalue self)
    (else
      (return false null))))

(fn `SetCameraPitchFromZoom`
  (`SceneComponent.K2_SetRelativeRotation` (`self.SpringArm`) (`KismetMathLibrary.MakeRotator` (.roll (`SceneComponent.RelativeRotation` (`self.SpringArm`))) (`KismetMathLibrary.Lerp` (`self.CameraMinDistancePitch`) (`self.CameraMaxDistancePitch`) (/ (- (`SpringArmComponent.TargetArmLength` (`self.SpringArm`)) (`self.CameraMinDistance`)) (- (`self.CameraMaxDistance`) (`self.CameraMinDistance`)))) (.yaw (`SceneComponent.RelativeRotation` (`self.SpringArm`)))) false false))

(fn `SetCameraTargetYaw`
  (if (`self.CameraYawMousePressed`)
    (`|ExecutionSequence`
      (:`then_0`
        (bind _returnvalue (`WidgetLayoutLibrary.GetMousePositionOnViewport`))
        (bind _returnvalue_2 (`self.GetCameraYawOffset` (- _returnvalue (`self.CameraYawClickOrigin`))))
        (bind _returnvalue_3 (+ (.yaw (`SceneComponent.RelativeRotation` (`self.SpringArm`))) _returnvalue_2))
        (`/Engine/EditorBlueprintResources/StandardMacros.CompareFloat` (`KismetMathLibrary.Abs` _returnvalue_3) (`self.CameraMaxYaw`)
          (:`<`
            (`SceneComponent.K2_SetRelativeRotation` (`self.SpringArm`) (`KismetMathLibrary.MakeRotator` (.roll (`SceneComponent.RelativeRotation` (`self.SpringArm`))) (.pitch (`SceneComponent.RelativeRotation` (`self.SpringArm`))) _returnvalue_3) false false))))
      (:`then_1`
        (bind _returnvalue_4 (`WidgetLayoutLibrary.GetMousePositionOnViewport`))
        (set `self.CameraYawClickOrigin` _returnvalue_4)))))

(fn `UserConstructionScript`
  (`self.SetCameraPitchFromZoom`))