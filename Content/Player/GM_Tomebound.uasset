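; Tomebound game mode that tracks a chain of tutorial missions in a Missions array of structs.
; Each UpdateMission function changes its mission's state and, unless the GameInstance flags that step completed, activates the next and sets the flag.
; ActivateMission writes the new state into the array and calls ShowMission on the training UI.
; UpdateMission3 also flags all tutorials completed before calling UpdateMission4, so that call skips activating mission 4.
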(event `self.ReceiveBeginPlay`)

(fn `activateMission`
  (params (Mission :type Integer))
  (bind _structout (setmembers `/Game/Systems/Tutorial/S_Mission` :`StructRef` (`|GetArrayItem` (`self.missions`) Mission) :`State` "NewEnumerator1"))
  (`KismetArrayLibrary.Array_Set` (`self.missions`) Mission _structout)
  (`/Game/Widgets/WBP_TrainUI.showMission` (`/Game/Player/PC_Player.trainUIRef` (`/Game/Systems/Tutorial/BPL_Tuto.castPlayerController`))))

(fn `updateMission1`
  (bind _asbp_player (cast `/Game/Player/BP_Player` (`GameplayStatics.GetPlayerCharacter` 0)))
  (set `/Game/Player/BP_Player.IsCameraTutoCompl?` true _asbp_player)
  (setmembers `/Game/Systems/Tutorial/S_Mission` :`StructRef` (`|GetArrayItem` (`self.missions`)) :`State` "NewEnumerator2")
  (bind _asgame_instance_tomebound (cast `/Game/Utilities/GameInstance/GameInstance_Tomebound` (`GameplayStatics.GetGameInstance`)))
  (if (not (`/Game/Utilities/GameInstance/GameInstance_Tomebound.tuto1Completed` _asgame_instance_tomebound))
    (`self.activateMission` 1)
    (set `/Game/Utilities/GameInstance/GameInstance_Tomebound.tuto1Completed` true _asgame_instance_tomebound)))

(fn `updateMission2`
  (set `self.IsMovingTutoCompl?` true)
  (setmembers `/Game/Systems/Tutorial/S_Mission` :`StructRef` (`|GetArrayItem` (`self.missions`) 1) :`State` "NewEnumerator2")
  (bind _asgame_instance_tomebound (cast `/Game/Utilities/GameInstance/GameInstance_Tomebound` (`GameplayStatics.GetGameInstance`)))
  (if (not (`/Game/Utilities/GameInstance/GameInstance_Tomebound.tuto2Completed` _asgame_instance_tomebound))
    (`self.activateMission` 2)
    (set `/Game/Utilities/GameInstance/GameInstance_Tomebound.tuto2Completed` true _asgame_instance_tomebound)))

(fn `updateMission3`
  (setmembers `/Game/Systems/Tutorial/S_Mission` :`StructRef` (`|GetArrayItem` (`self.missions`) 2) :`State` "NewEnumerator2")
  (bind _asgame_instance_tomebound (cast `/Game/Utilities/GameInstance/GameInstance_Tomebound` (`GameplayStatics.GetGameInstance`)))
  (if (not (`/Game/Utilities/GameInstance/GameInstance_Tomebound.tuto3Completed` _asgame_instance_tomebound))
    (`self.activateMission` 3)
    (bind _asbp_player (cast `/Game/Player/BP_Player` (`GameplayStatics.GetPlayerCharacter` 0)))
    (set `/Game/Player/BP_Player.IsAffinityTutoCompl?` true _asbp_player)
    (set `/Game/Utilities/GameInstance/GameInstance_Tomebound.tuto3Completed` true _asgame_instance_tomebound)
    (bind _asgame_instance_tomebound_2 (cast `/Game/Utilities/GameInstance/GameInstance_Tomebound` (`GameplayStatics.GetGameInstance`)))
    (set `/Game/Utilities/GameInstance/GameInstance_Tomebound.tuto4Completed` true _asgame_instance_tomebound_2)
    (set `/Game/Utilities/GameInstance/GameInstance_Tomebound.allTutoCompleted` true _asgame_instance_tomebound_2)
    (`self.updateMission4`)))

(fn `updateMission4`
  (setmembers `/Game/Systems/Tutorial/S_Mission` :`StructRef` (`|GetArrayItem` (`self.missions`) 3) :`State` "NewEnumerator2")
  (set `self.IsTutoKeyCompl?` true)
  (bind _asgame_instance_tomebound (cast `/Game/Utilities/GameInstance/GameInstance_Tomebound` (`GameplayStatics.GetGameInstance`)))
  (if (not (`/Game/Utilities/GameInstance/GameInstance_Tomebound.tuto4Completed` _asgame_instance_tomebound))
    (`self.activateMission` 4)
    (set `/Game/Utilities/GameInstance/GameInstance_Tomebound.tuto4Completed` true _asgame_instance_tomebound)))

(fn `UserConstructionScript`)