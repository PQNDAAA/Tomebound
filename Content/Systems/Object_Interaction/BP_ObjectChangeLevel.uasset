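; BP_ObjectChangeLevel is an interaction actor that sends the game to the persistent gameplay level when the player touches it.
; On any actor overlap it calls the parent handler, prints a debug "Hello", then checks whether its Collider overlaps player character 0.
; If so, it waits briefly and opens LVL_Persistent_Gameplay by name, with the destination hard-coded.
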(event `self.ReceiveActorBeginOverlap`
  (params (OtherActor :type "Actor Object Reference"))
  (`parent.ReceiveActorBeginOverlap` OtherActor)
  (`KismetSystemLibrary.PrintString` "Hello")
  (if (`PrimitiveComponent.IsOverlappingActor` (`self.Collider`) (`GameplayStatics.GetPlayerCharacter` 0))
    (`KismetSystemLibrary.Delay` 0.2)
    (`GameplayStatics.OpenLevel` "LVL_Persistent_Gameplay")))

(fn `UserConstructionScript`
  (`parent.UserConstructionScript`))