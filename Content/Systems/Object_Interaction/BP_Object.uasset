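; BP_Object is an interactable world object that shows a text dialog when clicked from nearby.
; Box overlap toggles its input and a gate, so a left click only counts in range and when the cursor trace hits an ObjectActor-tagged actor.
; The click disables pawn input, opens WBP_ObjectDialog with DialogText and prints a debug message.
; The stored widget reference blocks duplicate dialogs until ResetDialog clears it.
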(event `Key|LeftMouseButton`
  (params (Key :type "Key Structure"))
  (bind (_bblockinghit _binitialoverlap _time _distance _location _impactpoint _normal _impactnormal _physmat _hitactor) (`GameplayStatics.BreakHitResult` (`PlayerController.GetHitResultUnderCursorByChannel` (`GameplayStatics.GetPlayerController` 0) "TraceTypeQuery1" true)))
  (:`Pressed`
    (`/Engine/EditorBlueprintResources/StandardMacros.IsValid` _hitactor
      (:`Is Valid`
        (if (and (`self.ActorHasTag` _hitactor "ObjectActor") (not (`KismetSystemLibrary.IsValid` (`self.ObjectDialogReference`))))
          (`/Engine/EditorBlueprintResources/StandardMacros.Gate` true :!label _label
            (:`Exit`
              (`self.DisableInput` (`GameplayStatics.GetPlayerPawn` 0) (`GameplayStatics.GetPlayerController` 0))
              (bind _returnvalue (`|CreateWidget` "/Game/Widgets/WBP_ObjectDialog.WBP_ObjectDialog_C" null self))
              (bind _output_get (set `self.ObjectDialogReference` _returnvalue))
              (`UserWidget.AddToViewport` _output_get 0)
              (`/Game/Utilities/Librairies/BFL_Main.SetDialogBlockOnWidget` (`/Game/Widgets/WBP_ObjectDialog.DialogBlock` (`self.ObjectDialogReference`)) (`self.dialogText`))
              (`/Game/Utilities/Librairies/BFL_Main.PrintDebugChat` (`|FormatText` "ObjectInteraction" self) "ObjectInteraction"))))))))

(event `self.Box.OnComponentBeginOverlap`
  (params (OverlappedComponent :type "PrimitiveComponent Object Reference") (OtherActor :type "Actor Object Reference") (OtherComp :type "PrimitiveComponent Object Reference") (OtherBodyIndex :type Integer) (bFromSweep :type Boolean) (SweepResult :type "HitResult Structure (by ref)"))
  (`self.EnableInput` (`GameplayStatics.GetPlayerController` 0))
  (goto _label :!via `Open`))

(event `self.Box.OnComponentEndOverlap`
  (params (OverlappedComponent :type "PrimitiveComponent Object Reference") (OtherActor :type "Actor Object Reference") (OtherComp :type "PrimitiveComponent Object Reference") (OtherBodyIndex :type Integer))
  (`self.DisableInput` (`GameplayStatics.GetPlayerController` 0))
  (goto _label :!via `Close`))

(fn `ResetDialog`
  (set `self.ObjectDialogReference` null))

(fn `UserConstructionScript`)