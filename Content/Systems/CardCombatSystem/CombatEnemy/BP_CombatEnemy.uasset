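; BP_CombatEnemy is an enemy actor for the card combat system, defined by a data table row.
; On BeginPlay it loads its combat struct from that row, sets its health, and fills its name and health bar widgets.
; AnyDamage passes incoming damage through a TakeDamage call, subtracts the result from Health, updates the health bar, and prints the new value.
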(event `self.ReceiveBeginPlay`
  ;[1 1 1] Setup
  (`self.SetupEnemy`)
  (`self.SetEnemyNameOnWidget`)
  (`self.SetEnemyHealthOnWidget`))

(event `self.ReceiveAnyDamage`
  (params (Damage :type "Float (single-precision)") (DamageType :type "DamageType Object Reference") (InstigatedBy :type "Controller Object Reference") (DamageCauser :type "Actor Object Reference"))
  (bind _returnhealth (`/Game/ProtoCards/UICards/BPFL_Cards.TakeDamage` (`self.Health`) Damage self))
  (bind _output_get (set `self.Health` (- (`self.Health`) _returnhealth)))
  (`self.SetEnemyHealthOnWidget`)
  (`KismetSystemLibrary.PrintString` (`KismetStringLibrary.Conv_DoubleToString` _output_get)))

(fn `SetEnemyHealthOnWidget`
  (bind _aswbp_enemy_health_bar (cast `/Game/Systems/CardCombatSystem/CombatEnemy/Widgets/WBP_EnemyHealthBar` (`WidgetComponent.GetWidget` (`self.Widget_HealthBar`))))
  (`ProgressBar.SetPercent` (`/Game/Systems/CardCombatSystem/CombatEnemy/Widgets/WBP_EnemyHealthBar.HealthBar` _aswbp_enemy_health_bar) (/ (`self.Health`) (`.MaxHealth_8_76B6087440513A2C8D5322B599CD9C53` (break `/Game/Systems/CardCombatSystem/CombatEnemy/S_CombatEnemy` (`self.S_CombatEnemy`))))))

(fn `SetEnemyNameOnWidget`
  (bind _aswbp_enemy_name (cast `/Game/Systems/CardCombatSystem/CombatEnemy/Widgets/WBP_EnemyName` (`WidgetComponent.GetWidget` (`self.Widget_EnemyName`))))
  (`TextBlock.SetText` (`/Game/Systems/CardCombatSystem/CombatEnemy/Widgets/WBP_EnemyName.enemyName` _aswbp_enemy_name) (`.Name_5_88EB5D1047D115D938D0D8B67869EF3F` (break `/Game/Systems/CardCombatSystem/CombatEnemy/S_CombatEnemy` (`self.S_CombatEnemy`)))))

(fn `SetupEnemy`
  (bind (_datatable _rowname) (break `DataTableRowHandle` (`self.Enemy`)))
  (bind _returnvalue (`|GetDataTableRow` _datatable _rowname)
    (:`then`
      (set `self.S_CombatEnemy` _returnvalue)
      (set `self.Health` (`.Health_6_98C8B5594D36B6AB6CD8ACB983AD8C6C` (break `/Game/Systems/CardCombatSystem/CombatEnemy/S_CombatEnemy` (`self.S_CombatEnemy`)))))))

(fn `UserConstructionScript`)