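; Enemy actor for the card combat system, initialised from a data table row that supplies its name, health and damage.
; Combat events heal it, attack the player or deal multiplied damage, each showing feedback text from DT_CardEnemyAction.
; Healing also clears the player's block and avoid flags.
; Incoming damage updates the health bar or removes the enemy at zero, while CheckHealth tests health against a ratio threshold.
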(event `/Game/Systems/CardCombatSystem/CardCombat/AI/Interface/BI_EnemyCombat.CombatHeal`
  (bind _asbp_card_player (`/Game/Systems/CardCombatSystem/CardCombat/Cards/Libraries/BFL_Cards.GetCardPlayer`))
  (bind (_health _name _maxhealth) (break `/Game/Systems/CardCombatSystem/CardCombat/AI/Structure/S_CardEnemy` (`self.S_CombatEnemy`)))
  ;[1 1 1] Heal
  (`KismetSystemLibrary.PrintString` "Health")
  (set `self.Health` (+ (`self.Health`) 2.0))
  (`/Game/Systems/CardCombatSystem/CardCombat/Cards/Libraries/BFL_Cards.SetHealthBar` (`self.Widget_HealthBar`) (`self.Health`) _maxhealth)
  (bind _returnvalue (`|GetDataTableRow` "/Game/Systems/CardCombatSystem/CardCombat/AI/Datatable/DT_CardEnemyAction.DT_CardEnemyAction" "Heal")
    (:`then`
      (bind _returnvalue_2 (`|CreateWidget` "/Game/Systems/CardCombatSystem/CardCombat/AI/Widgets/WBP_UserFeedback.WBP_UserFeedback_C" null _name (`.Description_5_DB82D346428012641178AB8E8C49F01C` (break `/Game/Systems/CardCombatSystem/CardCombat/AI/Structure/S_CardEnemyAction` _returnvalue))))
      (`UserWidget.AddToViewport` _returnvalue_2 0)
      (set `/Game/Systems/CardCombatSystem/CardCombat/Player/BP_Card_Player.BlockDamage?` false _asbp_card_player)
      (set `/Game/Systems/CardCombatSystem/CardCombat/Player/BP_Card_Player.AvoidAttack?` false _asbp_card_player))))

(event `/Game/Systems/CardCombatSystem/CardCombat/AI/Interface/BI_EnemyCombat.CombatAttack`
  (bind _asbp_card_player (`/Game/Systems/CardCombatSystem/CardCombat/Cards/Libraries/BFL_Cards.GetCardPlayer`))
  (bind (_health _name _maxhealth _damage) (break `/Game/Systems/CardCombatSystem/CardCombat/AI/Structure/S_CardEnemy` (`self.S_CombatEnemy`)))
  ;[1 1 1] Attack
  (`KismetSystemLibrary.PrintString` "Attack")
  (`/Game/Systems/CardCombatSystem/CardCombat/Cards/Libraries/BFL_Cards.DealDamage` (`/Game/Systems/CardCombatSystem/CardCombat/Player/BP_Card_Player.WidgetFeedbackDamage` _asbp_card_player) _damage _asbp_card_player self)
  (bind _returnvalue (`|GetDataTableRow` "/Game/Systems/CardCombatSystem/CardCombat/AI/Datatable/DT_CardEnemyAction.DT_CardEnemyAction" "Attack")
    (:`then`
      (bind _returnvalue_2 (`|CreateWidget` "/Game/Systems/CardCombatSystem/CardCombat/AI/Widgets/WBP_UserFeedback.WBP_UserFeedback_C" null _name (`.Description_5_DB82D346428012641178AB8E8C49F01C` (break `/Game/Systems/CardCombatSystem/CardCombat/AI/Structure/S_CardEnemyAction` _returnvalue))))
      (`UserWidget.AddToViewport` _returnvalue_2 0))))

(event `/Game/Systems/CardCombatSystem/CardCombat/AI/Interface/BI_EnemyCombat.CombatBuff`
  (params (multiplier :type "Float (double-precision)"))
  (bind _asbp_card_player (`/Game/Systems/CardCombatSystem/CardCombat/Cards/Libraries/BFL_Cards.GetCardPlayer`))
  (bind (_health _name _maxhealth _damage) (break `/Game/Systems/CardCombatSystem/CardCombat/AI/Structure/S_CardEnemy` (`self.S_CombatEnemy`)))
  ;[1 1 1] Buff
  (`KismetSystemLibrary.PrintString` "Buff")
  (`/Game/Systems/CardCombatSystem/CardCombat/Cards/Libraries/BFL_Cards.DealDamage` (`/Game/Systems/CardCombatSystem/CardCombat/Player/BP_Card_Player.WidgetFeedbackDamage` _asbp_card_player) (* _damage multiplier) _asbp_card_player self)
  (bind _returnvalue (`|GetDataTableRow` "/Game/Systems/CardCombatSystem/CardCombat/AI/Datatable/DT_CardEnemyAction.DT_CardEnemyAction" "Buff")
    (:`then`
      (bind _returnvalue_2 (`|CreateWidget` "/Game/Systems/CardCombatSystem/CardCombat/AI/Widgets/WBP_UserFeedback.WBP_UserFeedback_C" null _name (`.Description_5_DB82D346428012641178AB8E8C49F01C` (break `/Game/Systems/CardCombatSystem/CardCombat/AI/Structure/S_CardEnemyAction` _returnvalue))))
      (`UserWidget.AddToViewport` _returnvalue_2 0))))

(event `self.ReceiveBeginPlay`
  ;[1 1 1] Setup
  (`self.SetupEnemy`)
  (`/Game/Systems/CardCombatSystem/CardCombat/Cards/Libraries/BFL_Cards.SetHealthBar` (`self.Widget_HealthBar`) (`self.Health`) (`.MaxHealth_8_76B6087440513A2C8D5322B599CD9C53` (break `/Game/Systems/CardCombatSystem/CardCombat/AI/Structure/S_CardEnemy` (`self.S_CombatEnemy`)))))

(event `self.ReceiveAnyDamage`
  (params (Damage :type "Float (single-precision)") (DamageType :type "DamageType Object Reference") (InstigatedBy :type "Controller Object Reference") (DamageCauser :type "Actor Object Reference"))
  (bind _widget_healthbar (`self.Widget_HealthBar`))
  (bind _health (`self.Health`))
  (bind (_health_2 _name _maxhealth) (break `/Game/Systems/CardCombatSystem/CardCombat/AI/Structure/S_CardEnemy` (`self.S_CombatEnemy`)))
  ;[1 1 1] Take Damage
  (bind _returnhealth (`/Game/Systems/CardCombatSystem/CardCombat/Cards/Libraries/BFL_Cards.TakeDamage` (`self.Health`) Damage self))
  (set `self.Health` _returnhealth)
  (if (<= (`self.Health`) 0.0)
    (`/Game/Systems/CardCombatSystem/CardCombat/Cards/Libraries/BFL_Cards.RemoveActor` _widget_healthbar _health _maxhealth self)
    (else
      (`/Game/Systems/CardCombatSystem/CardCombat/Cards/Libraries/BFL_Cards.SetHealthBar` _widget_healthbar _health _maxhealth))))

(fn `CheckHealth`
  (params (HealthCheckRange :type "Float (double-precision)"))
  (returns (`isValid?` :type Boolean))
  (return (<= (/ (`self.Health`) (`.MaxHealth_8_76B6087440513A2C8D5322B599CD9C53` (break `/Game/Systems/CardCombatSystem/CardCombat/AI/Structure/S_CardEnemy` (`self.S_CombatEnemy`)))) HealthCheckRange)))

(fn `SetEnemyNameOnWidget`
  (bind _aswbp_enemy_name (cast `/Game/Systems/CardCombatSystem/CardCombat/AI/Widgets/WBP_EnemyName` (`WidgetComponent.GetWidget` (`self.Widget_EnemyName`))))
  (`TextBlock.SetText` (`/Game/Systems/CardCombatSystem/CardCombat/AI/Widgets/WBP_EnemyName.enemyName` _aswbp_enemy_name) (`.Name_5_88EB5D1047D115D938D0D8B67869EF3F` (break `/Game/Systems/CardCombatSystem/CardCombat/AI/Structure/S_CardEnemy` (`self.S_CombatEnemy`)))))

(fn `SetupEnemy`
  (bind (_datatable _rowname) (break `DataTableRowHandle` (`self.Enemy`)))
  (bind _returnvalue (`|GetDataTableRow` _datatable _rowname)
    (:`then`
      (set `self.S_CombatEnemy` _returnvalue)
      (set `self.Health` (`.Health_6_98C8B5594D36B6AB6CD8ACB983AD8C6C` (break `/Game/Systems/CardCombatSystem/CardCombat/AI/Structure/S_CardEnemy` (`self.S_CombatEnemy`))))
      (`self.SetEnemyNameOnWidget`))))

(fn `UserConstructionScript`)