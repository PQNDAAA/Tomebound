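; BP_Author is an actor in the card combat system that tracks a police bar and can carry out a police raid on the card player.
; AddPointPoliceBar accumulates points and updates the progress bar and points/max text in its WBP_PoliceBar widget component.
; CheckPoliceBar reports whether points exactly equal the maximum, and CombatPoliceRaid deals a very large fixed hit to the card player through DealDamage.
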(event `/Game/Systems/CardCombatSystem/CardCombat/AI/Interface/BI_EnemyCombat.AddPointPoliceBar`
  (params (nbPoint :type "Float (double-precision)"))
  (bind _aswbp_police_bar (cast `/Game/Systems/CardCombatSystem/CardCombat/AI/Widgets/WBP_PoliceBar` (`WidgetComponent.GetUserWidgetObject` (`self.Widget_PoliceBar`)) :!pure true))
  (bind _output_get (set `self.policeBarPoint` (+ (`self.policeBarPoint`) nbPoint)))
  (`ProgressBar.SetPercent` (`/Game/Systems/CardCombatSystem/CardCombat/AI/Widgets/WBP_PoliceBar.policeBar` _aswbp_police_bar) (/ _output_get (`self.maxPoliceBar`)))
  (`TextBlock.SetText` (`/Game/Systems/CardCombatSystem/CardCombat/AI/Widgets/WBP_PoliceBar.policeBarTxt` _aswbp_police_bar) (`|FormatText` "{P}/{M}" (`self.policeBarPoint`) (`self.maxPoliceBar`))))

(event `/Game/Systems/CardCombatSystem/CardCombat/AI/Interface/BI_EnemyCombat.CombatPoliceRaid`
  (bind _asbp_card_player (`/Game/Systems/CardCombatSystem/CardCombat/Cards/Libraries/BFL_Cards.GetCardPlayer`))
  (`self.DealDamage` (`/Game/Systems/CardCombatSystem/CardCombat/BP_Entity.Widget_FeedbackDamage` _asbp_card_player) 1000.0 _asbp_card_player self))

(fn `CheckPoliceBar`
  (returns (`policeBarIsFull?` :type Boolean))
  (if (== (`self.policeBarPoint`) (`self.maxPoliceBar`))
    (return true)
    (else
      (return false))))

(fn `UserConstructionScript`
  (`parent.UserConstructionScript`))