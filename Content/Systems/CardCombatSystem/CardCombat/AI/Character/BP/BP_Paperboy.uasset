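; Paperboy enemy for card combat, likely a boss, whose spells disrupt the player's cards.
; RandomSpell makes a weighted roll between Cornered (randomizes card mana), PublicOpinion (triggers a random hand card with itself as enemy reference) and Confused (replaces the hand), returning the resulting intention.
; CombatBuff scales its multiplier with hand size.
; Actions play sounds and data-table Niagara effects; spells also swap sprites, reset by timer.
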(event `/Game/Systems/CardCombatSystem/CardCombat/AI/Interface/BI_EnemyCombat.CombatBuff`
  ;[1 1 1] BUFF
  (set `self.buffMultiplier` (`KismetMathLibrary.Conv_IntToDouble` (`KismetArrayLibrary.Array_Length` (`/Game/Systems/CardCombatSystem/CardCombat/Cards/Widgets/WBP_CardHand.CardWidgetRef` (`/Game/Systems/CardCombatSystem/CardCombat/Cards/Widgets/WBP_CardCombatHUD.W_CardHand` (`/Game/Systems/CardCombatSystem/CardCombat/Player/BP_CardGameMode.WBP_CombatHUD_Reference` (`/Game/Systems/CardCombatSystem/CardCombat/Cards/Libraries/BFL_Cards.Get Card Gamemode`)))))))
  (`parent.CombatBuff`)
  (`self.SetNiagaraFromDataTable` "/Game/Systems/CardCombatSystem/CardCombat/FX/Datatable/DT_BossFX.DT_BossFX" "PaperBoyAttack" (`self.Niagara`))
  (`GameplayStatics.PlaySound2D` (`self.attackSound`) 1.0 1.0 0.0 null null))

(event `/Game/Systems/CardCombatSystem/CardCombat/AI/Interface/BI_EnemyCombat.Cornered`
  ;[1 1 1] Cornered
  (bind _outactors (`GameplayStatics.GetAllActorsOfClass` "/Game/Systems/CardCombatSystem/CardCombat/Cards/BlueprintType/BP_CardBase.BP_CardBase_C"))
  (for _array_element _outactors
    (set `/Game/Systems/CardCombatSystem/CardCombat/Cards/BlueprintType/BP_CardBase.Mana` (`KismetMathLibrary.RandomIntegerInRange` 0 4) _array_element))
  (`self.SetSprite` "/Game/Systems/CardCombatSystem/CardCombat/Img/att2_paperboy_Sprite.att2_paperboy_Sprite")
  (`self.SetNiagaraFromDataTable` "/Game/Systems/CardCombatSystem/CardCombat/FX/Datatable/DT_BossFX.DT_BossFX" "PaperBoy_PublicOpinion" (`self.Niagara`))
  (`GameplayStatics.PlaySound2D` "/Game/Sounds/Feedback/Bosses_Sounds/Paperboy_Spell2_Cue.Paperboy_Spell2_Cue" 1.0 1.0 0.0 null null)
  (set `self.intentionValue` "NewEnumerator7"))

(event `/Game/Systems/CardCombatSystem/CardCombat/AI/Interface/BI_EnemyCombat.Confused`
  (bind _asbp_card_game_mode (`/Game/Systems/CardCombatSystem/CardCombat/Cards/Libraries/BFL_Cards.Get Card Gamemode`))
  (bind _wbp_combathud_reference (`/Game/Systems/CardCombatSystem/CardCombat/Player/BP_CardGameMode.WBP_CombatHUD_Reference` _asbp_card_game_mode))
  ;[1 1 1] Confused
  (`/Game/Systems/CardCombatSystem/CardCombat/Cards/Widgets/WBP_CardHand.DeleteAllCards` (`/Game/Systems/CardCombatSystem/CardCombat/Cards/Widgets/WBP_CardCombatHUD.W_CardHand` _wbp_combathud_reference))
  (`/Game/Systems/CardCombatSystem/CardCombat/Cards/Libraries/BFL_Cards.CreateCards` 0 (- (`/Game/Systems/CardCombatSystem/CardCombat/Player/BP_CardGameMode.maxCardCount` _asbp_card_game_mode) 1) _wbp_combathud_reference)
  (`self.SetSprite` "/Game/Systems/CardCombatSystem/CardCombat/Img/att3_paperboy_Sprite.att3_paperboy_Sprite")
  (`self.SetNiagara_Cornered`)
  (`GameplayStatics.PlaySound2D` "/Game/Sounds/Feedback/Bosses_Sounds/Paperboy_Spell3_Cue.Paperboy_Spell3_Cue" 1.0 1.0 0.0 null null)
  (set `self.intentionValue` "NewEnumerator9"))

(event `/Game/Systems/CardCombatSystem/CardCombat/AI/Interface/BI_EnemyCombat.PublicOpinion`
  (bind _asbp_card_controller (cast `/Game/Systems/CardCombatSystem/CardCombat/Player/BP_CardController` (`GameplayStatics.GetPlayerController` 0) :!pure true))
  ;[1 1 1] PublicOpinion
  (set `/Game/Systems/CardCombatSystem/CardCombat/Player/BP_CardController.enemyReference` self _asbp_card_controller)
  (`/Game/Systems/CardCombatSystem/CardCombat/Cards/Widgets/WBP_Cards.DoCardAction` (`KismetArrayLibrary.Array_Random` (`/Game/Systems/CardCombatSystem/CardCombat/Cards/Widgets/WBP_CardHand.CardWidgetRef` (`/Game/Systems/CardCombatSystem/CardCombat/Cards/Widgets/WBP_CardCombatHUD.W_CardHand` (`/Game/Systems/CardCombatSystem/CardCombat/Player/BP_CardGameMode.WBP_CombatHUD_Reference` (`/Game/Systems/CardCombatSystem/CardCombat/Cards/Libraries/BFL_Cards.Get Card Gamemode`))))))
  (set `/Game/Systems/CardCombatSystem/CardCombat/Player/BP_CardController.enemyReference` null _asbp_card_controller)
  (`self.SetSprite` "/Game/Systems/CardCombatSystem/CardCombat/Img/att1_paperboy_Sprite.att1_paperboy_Sprite")
  (`self.SetNiagaraFromDataTable` "/Game/Systems/CardCombatSystem/CardCombat/FX/Datatable/DT_BossFX.DT_BossFX" "PaperBoy_Confused_Cast" (`self.Niagara`))
  (`GameplayStatics.PlaySound2D` "/Game/Sounds/Feedback/Bosses_Sounds/Bag_Rummaging_Cue.Bag_Rummaging_Cue" 1.0 1.0 0.0 null null)
  (set `self.intentionValue` "NewEnumerator8"))

(fn `RandomSpell`
  (returns (intentionValue :type "/Game/Systems/CardCombatSystem/CardCombat/AI/Enumeration/E_Action Enum"))
  (bind _spellrandomnumber (`self.spellRandomNumber`))
  (set `self.spellRandomNumber` (`KismetMathLibrary.RandomIntegerInRange` 0 100))
  (if (`KismetMathLibrary.InRange_IntInt` _spellrandomnumber 0 40 true false)
    (`/Game/Systems/CardCombatSystem/CardCombat/AI/Interface/BI_EnemyCombat.Cornered`)
    (`KismetSystemLibrary.K2_SetTimer` null "ResetSprite" 1.0 :!label _label)
    (return (`self.intentionValue`))
    (elif (`KismetMathLibrary.InRange_IntInt` _spellrandomnumber 40 80 true false)
      (`/Game/Systems/CardCombatSystem/CardCombat/AI/Interface/BI_EnemyCombat.PublicOpinion`)
      (goto _label)
      (elif (`KismetMathLibrary.InRange_IntInt` _spellrandomnumber 80 100)
        (`/Game/Systems/CardCombatSystem/CardCombat/AI/Interface/BI_EnemyCombat.Confused`)
        (goto _label)))))

(fn `SetNiagara_Cornered`
  (`self.SetNiagaraFromDataTable` "/Game/Systems/CardCombatSystem/CardCombat/FX/Datatable/DT_BossFX.DT_BossFX" "PaperBoy_Cornered_Cast" (`self.Niagara`))
  (`self.SetNiagaraFromDataTable` "/Game/Systems/CardCombatSystem/CardCombat/FX/Datatable/DT_BossFX.DT_BossFX" "PaperBoy_Cornered_Hit" (`/Game/Systems/CardCombatSystem/CardCombat/BP_Entity.Niagara` (`/Game/Systems/CardCombatSystem/CardCombat/Cards/Libraries/BFL_Cards.GetCardPlayer`))))

(fn `UserConstructionScript`
  (`parent.UserConstructionScript`))