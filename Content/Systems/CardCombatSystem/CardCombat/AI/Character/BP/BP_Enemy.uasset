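; BP_Enemy is a card-combat enemy that attacks, buff-attacks, heals or hurts itself, and tracks its own health.
; Setup loads stats from a data-table row into health and name widgets; DT_CardEnemyAction supplies intention icons and action feedback text.
; Attacks damage the card player, while healing also clears the player's block and avoid flags.
; Incoming damage is reduced once when blocking is enabled and the blackboard intention matches, latched by EnemyBlockDamage.
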(event `/Game/Systems/CardCombatSystem/CardCombat/AI/Interface/BI_EnemyCombat.CombatAttackHimSelf`
  ;[1 1 1] Attack him self
  (bind _returnhealth (`self.TakeDamage` (`self.health`) 6.0))
  (set `self.health` _returnhealth)
  (`self.CheckHealth` (`self.Widget_HealthBar`) (`self.health`) (`.MaxHealth_8_76B6087440513A2C8D5322B599CD9C53` (break `/Game/Systems/CardCombatSystem/CardCombat/AI/Structure/S_CardEnemy` (`self.S_CombatEnemy`))) self))

(event `/Game/Systems/CardCombatSystem/CardCombat/AI/Interface/BI_EnemyCombat.CombatHeal`
  (bind _asbp_card_player (`/Game/Systems/CardCombatSystem/CardCombat/Cards/Libraries/BFL_Cards.GetCardPlayer`))
  (bind (_health _name _maxhealth) (break `/Game/Systems/CardCombatSystem/CardCombat/AI/Structure/S_CardEnemy` (`self.S_CombatEnemy`)))
  ;[1 1 1] Heal
  (`KismetSystemLibrary.PrintString` "Health")
  (set `self.health` (+ (`self.health`) 2.0))
  (`self.SetHealthBar` (`self.Widget_HealthBar`) (`self.health`) _maxhealth)
  (bind _returnvalue (`|GetDataTableRow` "/Game/Systems/CardCombatSystem/CardCombat/AI/Datatable/DT_CardEnemyAction.DT_CardEnemyAction" "Heal")
    (:`then`
      (bind _returnvalue_2 (`|CreateWidget` "/Game/Systems/CardCombatSystem/CardCombat/AI/Widgets/WBP_UserFeedback.WBP_UserFeedback_C" null _name (`.Description_5_DB82D346428012641178AB8E8C49F01C` (break `/Game/Systems/CardCombatSystem/CardCombat/AI/Structure/S_CardEnemyAction` _returnvalue))))
      (`UserWidget.AddToViewport` _returnvalue_2 0)
      (set `/Game/Systems/CardCombatSystem/CardCombat/Player/BP_Card_Player.BlockDamage?` false _asbp_card_player)
      (set `/Game/Systems/CardCombatSystem/CardCombat/Player/BP_Card_Player.AvoidAttack?` false _asbp_card_player))))

(event `/Game/Systems/CardCombatSystem/CardCombat/AI/Interface/BI_EnemyCombat.CombatAttack`
  (bind _asbp_card_player (`/Game/Systems/CardCombatSystem/CardCombat/Cards/Libraries/BFL_Cards.GetCardPlayer`))
  (bind (_health _name _maxhealth _damage) (break `/Game/Systems/CardCombatSystem/CardCombat/AI/Structure/S_CardEnemy` (`self.S_CombatEnemy`)))
  ;[1 1 1] Attack
  (`KismetSystemLibrary.PrintString` "Attack")
  (bind _output_get (set `self.applyDamage` _damage))
  (`self.DealDamage` (`/Game/Systems/CardCombatSystem/CardCombat/BP_Entity.Widget_FeedbackDamage` _asbp_card_player) _output_get _asbp_card_player self)
  (bind _returnvalue (`|GetDataTableRow` "/Game/Systems/CardCombatSystem/CardCombat/AI/Datatable/DT_CardEnemyAction.DT_CardEnemyAction" "Attack")
    (:`then`
      (bind _returnvalue_2 (`|CreateWidget` "/Game/Systems/CardCombatSystem/CardCombat/AI/Widgets/WBP_UserFeedback.WBP_UserFeedback_C" null _name (`.Description_5_DB82D346428012641178AB8E8C49F01C` (break `/Game/Systems/CardCombatSystem/CardCombat/AI/Structure/S_CardEnemyAction` _returnvalue))))
      (`UserWidget.AddToViewport` _returnvalue_2 0)
      (`self.ResetApplyDamage` :!label _label))))

(event `/Game/Systems/CardCombatSystem/CardCombat/AI/Interface/BI_EnemyCombat.CombatBuff`
  (bind _asbp_card_player (`/Game/Systems/CardCombatSystem/CardCombat/Cards/Libraries/BFL_Cards.GetCardPlayer`))
  (bind (_health _name _maxhealth _damage) (break `/Game/Systems/CardCombatSystem/CardCombat/AI/Structure/S_CardEnemy` (`self.S_CombatEnemy`)))
  ;[1 1 1] Buff
  (`KismetSystemLibrary.PrintString` "Buff")
  (bind _output_get (set `self.applyDamage` (* _damage (`self.buffMultiplier`))))
  (`self.DealDamage` (`/Game/Systems/CardCombatSystem/CardCombat/BP_Entity.Widget_FeedbackDamage` _asbp_card_player) _output_get _asbp_card_player self)
  (bind _returnvalue (`|GetDataTableRow` "/Game/Systems/CardCombatSystem/CardCombat/AI/Datatable/DT_CardEnemyAction.DT_CardEnemyAction" "Buff")
    (:`then`
      (bind _returnvalue_2 (`|CreateWidget` "/Game/Systems/CardCombatSystem/CardCombat/AI/Widgets/WBP_UserFeedback.WBP_UserFeedback_C" null _name (`.Description_5_DB82D346428012641178AB8E8C49F01C` (break `/Game/Systems/CardCombatSystem/CardCombat/AI/Structure/S_CardEnemyAction` _returnvalue))))
      (`UserWidget.AddToViewport` _returnvalue_2 0)
      (goto _label))))

(event `self.ReceiveBeginPlay`
  ;[1 1 1] Setup
  (`self.SetupEnemy`)
  (`self.SetHealthBar` (`self.Widget_HealthBar`) (`self.health`) (`.MaxHealth_8_76B6087440513A2C8D5322B599CD9C53` (break `/Game/Systems/CardCombatSystem/CardCombat/AI/Structure/S_CardEnemy` (`self.S_CombatEnemy`)))))

(event `self.ReceiveAnyDamage`
  (params (Damage :type "Float (single-precision)") (DamageType :type "DamageType Object Reference") (InstigatedBy :type "Controller Object Reference") (DamageCauser :type "Actor Object Reference"))
  (bind (_health _name _maxhealth _damage _buffmultiplier _blockdamage_ _blockdamagevalue) (break `/Game/Systems/CardCombatSystem/CardCombat/AI/Structure/S_CardEnemy` (`self.S_CombatEnemy`)))
  ;[1 1 1] Take Damage
  (if (and _blockdamage_ (== (`BlackboardComponent.GetValueAsEnum` (`AIBlueprintHelperLibrary.GetBlackboard` (`self.GetOwner`)) "intentionEnum") 0) (not (`self.enemyBlockDamage`)))
    (set `self.enemyBlockDamage` true)
    (set `self.receiveDamage` (- Damage _blockdamagevalue))
    (else
      (set `self.receiveDamage` Damage)))
  (bind _returnhealth (`self.TakeDamage` (`self.health`) (`self.receiveDamage`)))
  (set `self.health` _returnhealth)
  (`self.CheckHealth` (`self.Widget_HealthBar`) (`self.health`) (`.MaxHealth_8_76B6087440513A2C8D5322B599CD9C53` (break `/Game/Systems/CardCombatSystem/CardCombat/AI/Structure/S_CardEnemy` (`self.S_CombatEnemy`))) self))

(fn `CheckPoliceBar`
  (returns (`policeBarIsFull?` :type Boolean))
  (return false))

(fn `ResetApplyDamage`
  (set `self.applyDamage` 0.0))

(fn `SetEnemyIntention`
  (params (intentionEnum :type "/Game/Systems/CardCombatSystem/CardCombat/AI/Enumeration/E_Action Enum" :default "NewEnumerator0"))
  (bind _aswbp_enemy_intention (cast `/Game/Systems/CardCombatSystem/CardCombat/AI/Widgets/WBP_EnemyIntention` (`WidgetComponent.GetUserWidgetObject` (`self.Widget_Intention`)) :!pure true))
  (bind _outrownames (`DataTableFunctionLibrary.GetDataTableRowNames` "/Game/Systems/CardCombatSystem/CardCombat/AI/Datatable/DT_CardEnemyAction.DT_CardEnemyAction"))
  (for _array_element _outrownames
    (bind _returnvalue (`|GetDataTableRow` "/Game/Systems/CardCombatSystem/CardCombat/AI/Datatable/DT_CardEnemyAction.DT_CardEnemyAction" _array_element)
      (:`then`
        (bind (_action _description _image) (break `/Game/Systems/CardCombatSystem/CardCombat/AI/Structure/S_CardEnemyAction` _returnvalue))
        (if (`|EnumEquality` intentionEnum _action)
          (set `/Game/Systems/CardCombatSystem/CardCombat/AI/Widgets/WBP_EnemyIntention.intentionEnum` intentionEnum _aswbp_enemy_intention)
          (`Image.SetBrushFromTexture` (`/Game/Systems/CardCombatSystem/CardCombat/AI/Widgets/WBP_EnemyIntention.IntentionImage` _aswbp_enemy_intention) _image false))))))

(fn `SetEnemyNameOnWidget`
  (bind _aswbp_enemy_name (cast `/Game/Systems/CardCombatSystem/CardCombat/AI/Widgets/WBP_EnemyName` (`WidgetComponent.GetWidget` (`self.Widget_EnemyName`))))
  (`TextBlock.SetText` (`/Game/Systems/CardCombatSystem/CardCombat/AI/Widgets/WBP_EnemyName.enemyName` _aswbp_enemy_name) (`.Name_5_88EB5D1047D115D938D0D8B67869EF3F` (break `/Game/Systems/CardCombatSystem/CardCombat/AI/Structure/S_CardEnemy` (`self.S_CombatEnemy`)))))

(fn `SetupEnemy`
  (bind (_datatable _rowname) (break `DataTableRowHandle` (`self.Enemy`)))
  (bind (_health _name _maxhealth _damage _buffmultiplier) (break `/Game/Systems/CardCombatSystem/CardCombat/AI/Structure/S_CardEnemy` (`self.S_CombatEnemy`)))
  (bind _returnvalue (`|GetDataTableRow` _datatable _rowname)
    (:`then`
      (set `self.S_CombatEnemy` _returnvalue)
      (set `self.health` _health)
      (set `self.buffMultiplier` _buffmultiplier)
      (`self.SetEnemyNameOnWidget`))))

(fn `UserConstructionScript`)