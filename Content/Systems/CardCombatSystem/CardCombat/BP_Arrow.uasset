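; BP_Arrow is a card combat actor that draws an arrow along a spline using runtime spline meshes with an unlit material.
; AddSMSpline builds one Z-forward mesh per segment, and AddSMArrow adds another over the final segment, apparently the arrowhead.
; ClearSplines destroys those meshes and clears the spline points.
; The event graph and construction script are empty, and nothing here sets the points or calls these functions.
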(fn `addSMArrow`
  (bind _spline (`self.Spline`))
  (bind _returnvalue (- (`SplineComponent.GetNumberOfSplinePoints` (`self.Spline`)) 2))
  (bind (_location _tangent) (`SplineComponent.GetLocationAndTangentAtSplinePoint` _spline _returnvalue "Local"))
  (bind (_location_2 _tangent_2) (`SplineComponent.GetLocationAndTangentAtSplinePoint` _spline (+ _returnvalue 1) "Local"))
  (bind _returnvalue_2 (`AddComponent|NODE_AddSplineMeshComponent-3` :`bManualAttachment` true))
  (`PrimitiveComponent.SetMaterial` _returnvalue_2 0 "/Game/Systems/CardCombatSystem/CardCombat/M_ArrowUnlit.M_ArrowUnlit")
  (`SplineMeshComponent.SetForwardAxis` _returnvalue_2 "Z" true)
  (`KismetArrayLibrary.Array_Add` (`self.splineMeshes`) _returnvalue_2)
  (`SplineMeshComponent.SetStartAndEnd` _returnvalue_2 _location _tangent _location_2 _tangent_2 true))

(fn `addSMSpline`
  (bind _spline (`self.Spline`))
  (for _index (range (+ (- (`SplineComponent.GetNumberOfSplinePoints` (`self.Spline`)) 2) 1))
    (bind _returnvalue (`AddComponent|NODE_AddSplineMeshComponent-1` :`bManualAttachment` true))
    (`PrimitiveComponent.SetMaterial` _returnvalue 0 "/Game/Systems/CardCombatSystem/CardCombat/M_ArrowUnlit.M_ArrowUnlit")
    (`SplineMeshComponent.SetForwardAxis` _returnvalue "Z" true)
    (`KismetArrayLibrary.Array_Add` (`self.splineMeshes`) _returnvalue)
    (bind (_location _tangent) (`SplineComponent.GetLocationAndTangentAtSplinePoint` _spline _index "Local"))
    (bind (_location_2 _tangent_2) (`SplineComponent.GetLocationAndTangentAtSplinePoint` _spline (+ _index 1) "Local"))
    (`SplineMeshComponent.SetStartAndEnd` _returnvalue _location _tangent _location_2 _tangent_2 true)))

(fn `clearSplines`
  (bind _splinemeshes (`self.splineMeshes`))
  (`ActorComponent.K2_DestroyComponent` _splinemeshes)
  (`KismetArrayLibrary.Array_Clear` _splinemeshes)
  (`SplineComponent.ClearSplinePoints` (`self.Spline`) true))

(fn `UserConstructionScript`)