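; Background actor for the card combat system that shows a configurable texture on a plane.
; The construction script applies the texture through a dynamic instance of M_Background and scales the plane by screen resolution relative to ScreenWidth and ScreenHeight.
; Tick repeats the scaling on the plane's current scale, so any ratio other than one compounds every frame.
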(event `self.ReceiveBeginPlay`)

(event `self.ReceiveTick`
  (params (DeltaSeconds :type "Float (single-precision)"))
  (bind _plane (`self.Plane`))
  (bind (_relativescale3d_x _relativescale3d_y) (`KismetMathLibrary.BreakVector` (`SceneComponent.RelativeScale3D` _plane)))
  (bind _returnvalue (`GameUserSettings.GetGameUserSettings`))
  (bind (_x _y) (break `IntPoint` (`GameUserSettings.GetScreenResolution` _returnvalue)))
  (`SceneComponent.SetRelativeScale3D` _plane (`KismetMathLibrary.MakeVector` (* (/ _x (`self.ScreenWidth`)) _relativescale3d_x) (* (/ _y (`self.ScreenHeight`)) _relativescale3d_y) 1.0)))

(fn `UserConstructionScript`
  (bind _plane (`self.Plane`))
  (bind (_relativescale3d_x _relativescale3d_y) (`KismetMathLibrary.BreakVector` (`SceneComponent.RelativeScale3D` _plane)))
  (bind _returnvalue (`PrimitiveComponent.CreateDynamicMaterialInstance` (`self.Plane`) 0 "/Game/Systems/CardCombatSystem/CardCombat/Background/M_Background.M_Background" "None"))
  (`MaterialInstanceDynamic.SetTextureParameterValue` _returnvalue "Texture" (`self.BackgroundTexture`))
  (bind _returnvalue_2 (`GameUserSettings.GetGameUserSettings`))
  (bind (_x _y) (break `IntPoint` (`GameUserSettings.GetScreenResolution` _returnvalue_2)))
  (`SceneComponent.SetRelativeScale3D` _plane (`KismetMathLibrary.MakeVector` (* (/ _x (`self.ScreenWidth`)) _relativescale3d_x) (* (/ _y (`self.ScreenHeight`)) _relativescale3d_y) 1.0)))