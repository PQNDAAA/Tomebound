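; Base combat entity for the card combat system, providing shared health, damage and sprite helpers.
; DealDamage shows animated damage text and applies damage, while TakeDamage returns rounded health, ignoring negative damage.
; CheckHealth updates the health bar or destroys the target, opening the end-game widget unless the entity is an object.
; Sprite swaps trigger a timeline zoom that incrementally adds scale, and a helper feeds the shield widget.
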(event `ZoomSprite`
  (bind (_direction _tracksize) (`Timeline|Timeline_0` :!via `PlayFromStart`)
    (:`Update`
      (bind _returnvalue (`KismetMathLibrary.Lerp` 0.0 0.001 _tracksize))
      (set `self.scaleSprite` (+ (`SceneComponent.RelativeScale3D` (`self.PaperSprite`)) (`KismetMathLibrary.MakeVector` _returnvalue _returnvalue _returnvalue)))
      (`SceneComponent.SetRelativeScale3D` (`self.PaperSprite`) (`self.scaleSprite`)))
    (:`Finished`
      (`KismetSystemLibrary.PrintString` (`KismetTextLibrary.Conv_TextToString` (`|FormatText` "{name} : {v}" (`KismetSystemLibrary.GetDisplayName` self) (`KismetStringLibrary.Conv_VectorToString` (`self.scaleSprite`))))))))

(fn `CheckHealth`
  (params (HealthBarWidget :type "WidgetComponent Object Reference") (health :type "Float (double-precision)") (maxHealth :type "Float (double-precision)") (ActorTarget :type "Actor Object Reference"))
  (if (> health 0.0)
    (`self.SetHealthBar` HealthBarWidget health maxHealth)
    (else
      (`self.RemoveActor` HealthBarWidget health maxHealth ActorTarget))))

(fn `DealDamage`
  (params (FeedbackDamageWidgetReference :type "WidgetComponent Object Reference") (Damage :type "Float (double-precision)") (DamagedActor :type "Actor Object Reference") (DamageCauser :type "Actor Object Reference"))
  (`self.FeedbackDamage` FeedbackDamageWidgetReference Damage)
  (`GameplayStatics.ApplyDamage` DamagedActor Damage null DamageCauser))

(fn `FeedbackDamage`
  (params (FeedbackDamageWidgetReference :type "WidgetComponent Object Reference") (Damage :type "Float (double-precision)"))
  (bind _aswbp_feedback_damage (cast `/Game/Systems/CardCombatSystem/CardCombat/Widgets/WBP_FeedbackDamage` (`WidgetComponent.GetWidget` FeedbackDamageWidgetReference)))
  (bind _feedbackdamagetxt (`/Game/Systems/CardCombatSystem/CardCombat/Widgets/WBP_FeedbackDamage.feedbackDamageTxt` _aswbp_feedback_damage))
  (`TextBlock.SetText` _feedbackdamagetxt (`|FormatText` "-{damage}" Damage))
  (`Widget.SetVisibility` _feedbackdamagetxt "Visible")
  (`UserWidget.PlayAnimation` _aswbp_feedback_damage (`/Game/Systems/CardCombatSystem/CardCombat/Widgets/WBP_FeedbackDamage.feedbackDamage` _aswbp_feedback_damage) 0.0 1 "Forward" 1.0 false))

(fn `RemoveActor`
  (params (HealthBarWidget :type "WidgetComponent Object Reference") (Health :type "Float (double-precision)") (MaxHealth :type "Float (double-precision)") (ActorTarget :type "Actor Object Reference"))
  (locals (NewLocalVar :type "/Game/Systems/CardCombatSystem/CardCombat/Widgets/WBP_End Object Reference"))
  (`self.SetHealthBar` HealthBarWidget Health MaxHealth)
  (if (not (`self.isAnObject?`))
    (bind _returnvalue (`|CreateWidget` "/Game/Systems/CardCombatSystem/CardCombat/Widgets/WBP_End.WBP_End_C" null (`self.stateEndGameIfDead`)))
    (`UserWidget.AddToViewport` _returnvalue 0))
  (`self.K2_DestroyActor` ActorTarget))

(fn `ResetSprite`
  (`PaperSpriteComponent.SetSprite` (`self.PaperSprite`) (`self.baseSprite`)))

(fn `SetHealthBar`
  (params (HealthBarWidget :type "WidgetComponent Object Reference") (Health :type "Float (double-precision)") (MaxHealth :type "Float (double-precision)"))
  (locals (healthPercent :type "Float (double-precision)"))
  (set `local.healthPercent` (/ Health MaxHealth))
  (bind _aswbp_health_bar (cast `/Game/Systems/CardCombatSystem/CardCombat/Widgets/WBP_HealthBar` (`WidgetComponent.GetWidget` HealthBarWidget)))
  (`ProgressBar.SetPercent` (`/Game/Systems/CardCombatSystem/CardCombat/Widgets/WBP_HealthBar.HealthBar` _aswbp_health_bar) (`local.healthPercent`))
  (`TextBlock.SetText` (`/Game/Systems/CardCombatSystem/CardCombat/Widgets/WBP_HealthBar.healthTxt` _aswbp_health_bar) (`|FormatText` "{H}/{MH}" Health MaxHealth)))

(fn `SetShieldWidget`
  (params (shieldValue :type Integer))
  (bind _widgetshield (`self.WidgetShield`))
  (`/Engine/EditorBlueprintResources/StandardMacros.IsValid` _widgetshield
    (:`Is Valid`
      (set `/Game/Systems/CardCombatSystem/CardCombat/Cards/Widgets/WBP_Shield.shieldValue` shieldValue (cast `/Game/Systems/CardCombatSystem/CardCombat/Cards/Widgets/WBP_Shield` (`WidgetComponent.GetUserWidgetObject` _widgetshield) :!pure true)))))

(fn `SetSprite`
  (params (NewSprite :type "PaperSprite Object Reference"))
  (`PaperSpriteComponent.SetSprite` (`self.PaperSprite`) NewSprite)
  (`self.ZoomSprite`))

(fn `TakeDamage`
  (params (health :type "Float (double-precision)") (damage :type "Float (double-precision)"))
  (returns (returnHealth :type "Float (double-precision)"))
  (locals (finalHealth :type "Float (double-precision)"))
  (if (< damage 0.0)
    (bind _output_get (set `local.finalHealth` (- health 0.0)))
    (return (`KismetMathLibrary.Conv_IntToDouble` (`KismetMathLibrary.Round` _output_get)))
    (else
      (bind _output_get_2 (set `local.finalHealth` (- health damage)))
      (return (`KismetMathLibrary.Conv_IntToDouble` (`KismetMathLibrary.Round` _output_get_2))))))

(fn `UserConstructionScript`)