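; BP_Epiphany is the Epiphany card Blueprint in the card combat system.
; It overrides CardOnClicked, running the parent check first and then calling Inspiration on the card's player with its mana cost and itself.
; When Inspiration succeeds, the card adds investment damage and mastery stats.
; The click returns the Inspiration result, or false if the parent check fails.
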(event `self.ReceiveBeginPlay`
  (`parent.ReceiveBeginPlay`))

(fn `CardOnClicked`
  (returns (`isValid?` :type Boolean))
  (bind _isvalid_ (`parent.CardOnClicked`))
  (if _isvalid_
    (bind _isvalid__2 (`/Game/Systems/CardCombatSystem/CardCombat/Player/Interface/BI_PlayerCombat.Inspiration` (`/Game/Systems/CardCombatSystem/CardCombat/Cards/Libraries/BFL_Cards.GetCardPlayer`) (`self.Mana`) self))
    (if _isvalid__2
      (`self.AddInvestmentDamage`)
      (`self.AddMasteryStats`))
    (return _isvalid__2)
    (else
      (return false))))

(fn `UserConstructionScript`
  (`parent.UserConstructionScript`))