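; Patient Study is a block card in the card combat system, built on a parent card class.
; When the parent click check passes, it asks the card player to block for the truncated final value using its mana cost.
; A successful block triggers investment damage, mastery stat and Holy Bible mana hooks.
; The final value derives from the base value and mastery block bonus, which can be reset to zero.
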(event `self.ReceiveBeginPlay`
  (`parent.ReceiveBeginPlay`)
  (`self.UpdateCardValueDescription`))

(fn `CardOnClicked`
  (returns (`isValid?` :type Boolean))
  (bind _isvalid_ (`parent.CardOnClicked`))
  (if _isvalid_
    (bind _isvalid__2 (`/Game/Systems/CardCombatSystem/CardCombat/Player/BP_Card_Player.Block` (`/Game/Systems/CardCombatSystem/CardCombat/Cards/Libraries/BFL_Cards.GetCardPlayer`) (`KismetMathLibrary.FTrunc` (`self.finalDamage`)) (`self.Mana`) self))
    (if _isvalid__2
      (`self.AddInvestmentDamage`)
      (`self.AddMasteryStats`)
      (`self.AddManaHolyBible`))
    (return _isvalid__2)
    (else
      (return false))))

(fn `ResetMasteryStats`
  (set `self.masteryBlock` 0.0))

(fn `UpdateCardValueDescription`
  (returns (valueToUpdate :type "Float (double-precision)"))
  (`parent.UpdateCardValueDescription`)
  (bind _returnvalue (`self.SetFinalDamage` (`self.baseValue`) (`self.masteryBlock`)))
  (return _returnvalue))

(fn `UserConstructionScript`
  (`parent.UserConstructionScript`))