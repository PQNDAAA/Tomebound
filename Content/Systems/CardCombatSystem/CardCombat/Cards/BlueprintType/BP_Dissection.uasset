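; BP_Dissection is the Blueprint for the Dissection card in the card combat system.
; It overrides CardOnClicked and, when the parent check succeeds, sends the card player a DissectionMessage with a fixed mana bonus, the card's mana to remove and itself.
; It then calls the investment damage, mastery stats and Holy Bible mana helpers before returning success; otherwise it returns false.
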(fn `CardOnClicked`
  (returns (`isValid?` :type Boolean))
  (bind _isvalid_ (`parent.CardOnClicked`))
  (if _isvalid_
    (message `/Game/Systems/CardCombatSystem/CardCombat/Player/Interface/BI_PlayerCombat.Dissection` (`/Game/Systems/CardCombatSystem/CardCombat/Cards/Libraries/BFL_Cards.GetCardPlayer`) 3 (`self.Mana`) self)
    (`self.AddInvestmentDamage`)
    (`self.AddMasteryStats`)
    (`self.AddManaHolyBible`)
    (return true)
    (else
      (return false))))

(fn `UserConstructionScript`
  (`parent.UserConstructionScript`))