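; BP_Recognition is a card Blueprint for the card combat system, defining what happens when the Recognition card is clicked.
; Its CardOnClicked override runs the parent check first, then calls Recognition on the card player with the card's Mana.
; If that succeeds it calls IncreaseStats on the player, and the function returns whether the play succeeded.
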(fn `CardOnClicked`
  (returns (`isValid?` :type Boolean))
  (bind _asbp_card_player (`/Game/Systems/CardCombatSystem/CardCombat/Cards/Libraries/BFL_Cards.GetCardPlayer`))
  (bind _isvalid_ (`parent.CardOnClicked`))
  (if _isvalid_
    (bind _isvalid__2 (`/Game/Systems/CardCombatSystem/CardCombat/Player/Interface/BI_PlayerCombat.Recognition` _asbp_card_player (`self.Mana`)))
    (if _isvalid__2
      (`/Game/Systems/CardCombatSystem/CardCombat/Player/BP_Card_Player.Increase Stats` _asbp_card_player 1.0))
    (return _isvalid__2)
    (else
      (return false))))

(fn `UserConstructionScript`
  (`parent.UserConstructionScript`))