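; BP_AceUpTheSleeve is a card in the card combat system that gambles for mana when played.
; It overrides CardOnClicked and acts only if the parent implementation succeeds.
; It then grants the card's player a random amount of mana from a small range that includes zero, subtracts the card's own Mana cost, and returns success.
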(fn `CardOnClicked`
  (returns (`isValid?` :type Boolean))
  (bind _asbp_card_player (`/Game/Systems/CardCombatSystem/CardCombat/Cards/Libraries/BFL_Cards.GetCardPlayer`))
  (bind _isvalid_ (`parent.CardOnClicked`))
  (if _isvalid_
    (`/Game/Systems/CardCombatSystem/CardCombat/Player/BP_Card_Player.AddMana` _asbp_card_player (`KismetMathLibrary.RandomIntegerInRange` 0 5))
    (`/Game/Systems/CardCombatSystem/CardCombat/Player/BP_Card_Player.RemoveMana` _asbp_card_player (`self.Mana`) self)
    (return true)
    (else
      (return false))))

(fn `UserConstructionScript`
  (`parent.UserConstructionScript`))