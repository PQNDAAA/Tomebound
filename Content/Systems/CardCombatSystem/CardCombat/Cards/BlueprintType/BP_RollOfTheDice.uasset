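; Roll of the Dice card for the card combat system, dealing random damage at a mana cost.
; On click, it passes a rounded roll between the final min and max to the player's RollOfTheDice, adding investment, mastery and Holy Bible mana bonuses on success.
; Its damage range updates on BeginPlay.
; An uncalled-here helper lowers mana on one fixed card type, ignoring its type input and stopping at zero-mana matches.
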(event `self.ReceiveBeginPlay`
  (`parent.ReceiveBeginPlay`)
  (`self.UpdateCardRandomValueDescription`))

(fn `CardOnClicked`
  (returns (`isValid?` :type Boolean))
  (bind _isvalid_ (`parent.CardOnClicked`))
  (if _isvalid_
    (bind _isvalid__2 (`/Game/Systems/CardCombatSystem/CardCombat/Player/Interface/BI_PlayerCombat.RollOfTheDice` (`/Game/Systems/CardCombatSystem/CardCombat/Cards/Libraries/BFL_Cards.GetCardPlayer`) (`KismetMathLibrary.Conv_IntToDouble` (`KismetMathLibrary.Round` (`KismetMathLibrary.RandomFloatInRange` (`self.finalMinValue`) (`self.finalMaxValue`)))) (`self.Mana`) self))
    (if _isvalid__2
      (`self.AddInvestmentDamage`)
      (`self.AddMasteryStats`)
      (`self.AddManaHolyBible`))
    (return _isvalid__2)
    (else
      (return false))))

(fn `Decrease Type Mana`
  (params (cardType :type "/Game/Systems/CardCombatSystem/CardCombat/Cards/BlueprintType/Enum/E_CardType Enum" :default "NewEnumerator0") (manaToDecrease :type Integer :default 1))
  (bind _outactors (`GameplayStatics.GetAllActorsOfClass` "/Game/Systems/CardCombatSystem/CardCombat/Cards/BlueprintType/BP_CardBase.BP_CardBase_C"))
  (for _array_element _outactors
    (if (`|EnumEquality` (`.cardType_70_A092AFEC4C14968E7C724A968DCA6605` (break `/Game/Systems/CardCombatSystem/CardCombat/Cards/Structure/S_CardInfo` (`/Game/Systems/CardCombatSystem/CardCombat/Cards/BlueprintType/BP_CardBase.CardInfo` _array_element))) "NewEnumerator0")
      (bind _mana (`/Game/Systems/CardCombatSystem/CardCombat/Cards/BlueprintType/BP_CardBase.Mana` _array_element))
      (if (!= _mana 0)
        (set `/Game/Systems/CardCombatSystem/CardCombat/Cards/BlueprintType/BP_CardBase.Mana` (- _mana manaToDecrease) _array_element)
        (else
          (return))))))

(fn `UpdateCardRandomValueDescription`
  (returns (A :type "Float (double-precision)") (B :type "Float (double-precision)"))
  (`parent.UpdateCardRandomValueDescription`)
  (bind (_returnvaluemin _returnvaluemax) (`self.SetRandomDamage` (`self.minDamage`) (`self.maxDamage`) (`self.addtionalDamage`)))
  (return _returnvaluemin _returnvaluemax))

(fn `UserConstructionScript`
  (`parent.UserConstructionScript`))