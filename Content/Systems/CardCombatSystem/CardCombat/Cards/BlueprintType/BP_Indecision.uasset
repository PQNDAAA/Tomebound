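; BP_Indecision is a card in the card combat system that applies a mana malus to cards when played.
; It overrides CardOnClicked and adds its effect only when the parent click handler succeeds, passing that result back.
; AddManaMalus finds every BP_CardBase actor in the world, itself included, and sets its ManaMalus to a fixed value rather than incrementing it.
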(fn `AddManaMalus`
  (bind _outactors (`GameplayStatics.GetAllActorsOfClass` "/Game/Systems/CardCombatSystem/CardCombat/Cards/BlueprintType/BP_CardBase.BP_CardBase_C"))
  (for _array_element _outactors
    (set `/Game/Systems/CardCombatSystem/CardCombat/Cards/BlueprintType/BP_CardBase.manaMalus` 1 _array_element)))

(fn `CardOnClicked`
  (returns (`isValid?` :type Boolean))
  (bind _isvalid_ (`parent.CardOnClicked`))
  (if _isvalid_
    (`self.AddManaMalus`)
    (return true)
    (else
      (return false))))

(fn `UserConstructionScript`
  (`parent.UserConstructionScript`))