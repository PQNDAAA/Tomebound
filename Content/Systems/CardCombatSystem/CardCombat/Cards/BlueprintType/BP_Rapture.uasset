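; BP_Rapture is the Rapture card in the card combat system, zeroing the Mana of every other card when successfully played.
; CardOnClicked runs the parent check and, on success, calls ReduceAllMana, then the investment damage, mastery stat and Holy Bible mana functions.
; ReduceAllMana finds all BP_CardBase actors, skips itself, and sets each one's Mana to zero and Rapture flag to true.
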(fn `CardOnClicked`
  (returns (`isValid?` :type Boolean))
  (bind _isvalid_ (`parent.CardOnClicked`))
  (if _isvalid_
    (`self.ReduceAllMana`)
    (`self.AddInvestmentDamage`)
    (`self.AddMasteryStats`)
    (`self.AddManaHolyBible`)
    (return true)
    (else
      (return false))))

(fn `ReduceAllMana`
  (bind _outactors (`GameplayStatics.GetAllActorsOfClass` "/Game/Systems/CardCombatSystem/CardCombat/Cards/BlueprintType/BP_CardBase.BP_CardBase_C"))
  (for _array_element _outactors
    (if (!= _array_element self)
      (set `/Game/Systems/CardCombatSystem/CardCombat/Cards/BlueprintType/BP_CardBase.Mana` 0 _array_element)
      (set `/Game/Systems/CardCombatSystem/CardCombat/Cards/BlueprintType/BP_CardBase.rapture?` true _array_element))))

(fn `UserConstructionScript`
  (`parent.UserConstructionScript`))