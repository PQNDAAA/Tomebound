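; BP_Drunk is a card Blueprint in the card combat system that randomizes another card's mana when played.
; CardOnClicked runs the parent check first and, on success, calls SetInspirationRandomCard and AddInvestmentDamage, then returns true.
; Despite its name, SetInspirationRandomCard picks no random card: it gives the first other BP_CardBase actor found in the world a random Mana within a small range, then stops.
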(fn `CardOnClicked`
  (returns (`isValid?` :type Boolean))
  (bind _isvalid_ (`parent.CardOnClicked`))
  (if _isvalid_
    (`self.SetInspirationRandomCard`)
    (`self.AddInvestmentDamage`)
    (return true)
    (else
      (return false))))

(fn `SetInspirationRandomCard`
  (bind _outactors (`GameplayStatics.GetAllActorsOfClass` "/Game/Systems/CardCombatSystem/CardCombat/Cards/BlueprintType/BP_CardBase.BP_CardBase_C"))
  (for _array_element _outactors
    (if (!= _array_element self)
      (set `/Game/Systems/CardCombatSystem/CardCombat/Cards/BlueprintType/BP_CardBase.Mana` (`KismetMathLibrary.RandomIntegerInRange` 1 4) _array_element)
      (break))))

(fn `UserConstructionScript`
  (`parent.UserConstructionScript`))