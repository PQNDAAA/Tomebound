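; BP_HolyTouch is a combat card Blueprint for the Holy Touch card in the card combat system.
; On click, after the parent check passes, it calls the card player's HolyTouch with its mana cost, itself and its final damage.
; On success it adds investment damage, mastery stats and Holy Bible mana, and returns the result.
; Its description update recomputes final damage from attack and additional damage.
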(event `self.ReceiveBeginPlay`
  (`parent.ReceiveBeginPlay`))

(fn `CardOnClicked`
  (returns (`isValid?` :type Boolean))
  (bind _isvalid_ (`parent.CardOnClicked`))
  (if _isvalid_
    (bind _isvalid__2 (`/Game/Systems/CardCombatSystem/CardCombat/Player/Interface/BI_PlayerCombat.HolyTouch` (`/Game/Systems/CardCombatSystem/CardCombat/Cards/Libraries/BFL_Cards.GetCardPlayer`) (`self.Mana`) self (`self.finalDamage`)))
    (if _isvalid__2
      (`self.AddInvestmentDamage`)
      (`self.AddMasteryStats`)
      (`self.AddManaHolyBible`))
    (return _isvalid__2)
    (else
      (return false))))

(fn `UpdateCardValueDescription`
  (returns (valueToUpdate :type "Float (double-precision)"))
  (`parent.UpdateCardValueDescription`)
  (bind _returnvalue (`self.SetFinalDamage` (`self.attackDamage`) (`self.addtionalDamage`)))
  (return _returnvalue))

(fn `UserConstructionScript`
  (`parent.UserConstructionScript`))