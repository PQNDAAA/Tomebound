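; BP_Investment is a card in the card combat system that performs the Investment action when clicked.
; It overrides CardOnClicked and, if the parent check passes, calls Investment on the card's player with base plus additional attack damage, the mana cost and itself.
; On success it also calls IncreaseStats on that player, and it returns whether the action succeeded.
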(fn `CardOnClicked`
  (returns (`isValid?` :type Boolean))
  (bind _asbp_card_player (`/Game/Systems/CardCombatSystem/CardCombat/Cards/Libraries/BFL_Cards.GetCardPlayer`))
  (bind _isvalid_ (`parent.CardOnClicked`))
  (if _isvalid_
    (bind _isvalid__2 (`/Game/Systems/CardCombatSystem/CardCombat/Player/BP_Card_Player.Investment` _asbp_card_player (+ (`self.attackDamage`) (`self.addtionalDamage`)) (`self.Mana`) self))
    (if _isvalid__2
      (`/Game/Systems/CardCombatSystem/CardCombat/Player/BP_Card_Player.Increase Stats` _asbp_card_player 1.0))
    (return _isvalid__2)
    (else
      (return false))))

(fn `UserConstructionScript`
  (`parent.UserConstructionScript`))