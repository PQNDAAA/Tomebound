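; BP_Astronomy is an attack card in the card combat system whose damage grows with the current round number.
; AstronomyDamage adds the round number times a bonus to the base value, and the description update combines it with additional damage into the final damage, first computed on BeginPlay.
; A successful click sends an attack message to the card player, then applies investment damage, mastery stats and Holy Bible mana.
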(event `self.ReceiveBeginPlay`
  (`parent.ReceiveBeginPlay`)
  (`self.UpdateCardValueDescription`))

(fn `astronomyDamage`
  (params (attackBonus :type "Float (double-precision)"))
  (returns (returnValue :type "Float (double-precision)"))
  (return (+ (* attackBonus (`KismetMathLibrary.Conv_IntToDouble` (`/Game/Systems/CardCombatSystem/CardCombat/Player/BP_CardGameMode.roundNumber` (`/Game/Systems/CardCombatSystem/CardCombat/Cards/Libraries/BFL_Cards.Get Card Gamemode`)))) (`self.baseValue`))))

(fn `CardOnClicked`
  (returns (`isValid?` :type Boolean))
  (bind _isvalid_ (`parent.CardOnClicked`))
  (if _isvalid_
    (bind _isvalid__2 (message `/Game/Systems/CardCombatSystem/CardCombat/Player/Interface/BI_PlayerCombat.Attack` (`/Game/Systems/CardCombatSystem/CardCombat/Cards/Libraries/BFL_Cards.GetCardPlayer`) (`self.finalDamage`) (`self.Mana`) self))
    (if _isvalid__2
      (`self.AddInvestmentDamage`)
      (`self.AddMasteryStats`)
      (`self.AddManaHolyBible`))
    (return _isvalid__2)
    (else
      (return false))))

(fn `UpdateCardValueDescription`
  (returns (valueToUpdate :type "Float (double-precision)"))
  (`parent.UpdateCardValueDescription`)
  (bind _returnvalue (`self.SetFinalDamage` (`self.astronomyDamage` 2.0) (`self.addtionalDamage`)))
  (return _returnvalue))

(fn `UserConstructionScript`
  (`parent.UserConstructionScript`))