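; Holy Bible card for the card combat system, built around an accumulating mana bonus.
; When the parent click check passes, it sends the bonus to the card player's HolyBibleMessage and, on success, adds investment damage and mastery stats.
; AddManaBonus and ResetHolyBible grow or clear the bonus.
; The value description, refreshed on BeginPlay, feeds that bonus into the parent's final damage value.
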(event `self.ReceiveBeginPlay`
  (`parent.ReceiveBeginPlay`)
  (`self.UpdateCardValueDescription`))

(fn `AddManaBonus`
  (params (Amount :type Integer))
  (set `self.manaBonus` (+ (`self.manaBonus`) Amount)))

(fn `CardOnClicked`
  (returns (`isValid?` :type Boolean))
  (bind _isvalid_ (`parent.CardOnClicked`))
  (if _isvalid_
    (bind _isvalid__2 (message `/Game/Systems/CardCombatSystem/CardCombat/Player/Interface/BI_PlayerCombat.HolyBible` (`/Game/Systems/CardCombatSystem/CardCombat/Cards/Libraries/BFL_Cards.GetCardPlayer`) (`self.manaBonus`)))
    (if _isvalid__2
      (`self.AddInvestmentDamage`)
      (`self.AddMasteryStats`))
    (return _isvalid__2)
    (else
      (return false))))

(fn `ResetHolyBible`
  (set `self.manaBonus` 0))

(fn `UpdateCardValueDescription`
  (returns (valueToUpdate :type "Float (double-precision)"))
  (`parent.UpdateCardValueDescription`)
  (bind _returnvalue (`self.SetFinalDamage` (`KismetMathLibrary.Conv_IntToDouble` (`self.manaBonus`))))
  (return _returnvalue))

(fn `UserConstructionScript`
  (`parent.UserConstructionScript`))