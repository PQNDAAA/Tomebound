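; Player combatant (Mia) in the card combat system, holding health, mana, block, dodge and the card pool.
; SetupCards builds the pool from DT_Cards by status and Tome affinity, and ReshuffleCards subtracts cards in hand.
; Each card effect is a function that deals damage or changes state, spends mana and returns success.
; AnyDamage resolves dodge or block before updating health, with timed Paper2D sprite swaps for feedback.
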(event `self.ReceiveTick`
  (params (DeltaSeconds :type "Float (single-precision)")))

(event `Key|SpaceBar`
  (params (Key :type "Key Structure")))

(event `self.ReceiveBeginPlay`
  ;[1 1 1] Setup
  (`self.SetHealthBar` (`self.Widget_HealthBar`) (`self.health`) (`self.maxHealth`))
  (`/Game/Utilities/GameInstance/GameInstance_Tomebound.AccessToViewportDebugChat` (`/Game/Utilities/Librairies/BFL_Main.GetGameInstanceTomebound`)))

(event `self.ReceiveAnyDamage`
  (params (Damage :type "Float (single-precision)") (DamageType :type "DamageType Object Reference") (InstigatedBy :type "Controller Object Reference") (DamageCauser :type "Actor Object Reference"))
  ;[1 1 1] Take Damage
  (if (`self.BlockDamage?`)
    (`self.SetSprite` "/Game/Systems/CardCombatSystem/CardCombat/Img/CA_Art_Sprite_miahurt_Sprite.CA_Art_Sprite_miahurt_Sprite")
    (bind (_finaldamage _finalblock) (`self.BlockDamage` Damage (`KismetMathLibrary.Conv_IntToDouble` (`self.blockDamageStorage`))))
    (set `self.damage` _finaldamage)
    (set `self.blockDamageStorage` (`KismetMathLibrary.Round` _finalblock))
    (elif (`self.AvoidAttack?`)
      (`self.SetSprite` "/Game/Systems/CardCombatSystem/CardCombat/Img/CA_Art_Sprite_miadodge_Sprite.CA_Art_Sprite_miadodge_Sprite")
      (set `self.damage` 0.0)
      (else
        (`self.SetSprite` "/Game/Systems/CardCombatSystem/CardCombat/Img/CA_Art_Sprite_miahurt_Sprite.CA_Art_Sprite_miahurt_Sprite")
        (bind (_finaldamage_2 _finalblock_2) (`self.BlockDamage` Damage (`KismetMathLibrary.Conv_IntToDouble` (`self.blockDamageStorage`))))
        (set `self.damage` _finaldamage_2)
        (set `self.blockDamageStorage` (`KismetMathLibrary.Round` _finalblock_2)))))
  (bind _returnhealth (`self.TakeDamage` (`self.health`) (`self.damage`)))
  (set `self.health` _returnhealth)
  (`self.CheckHealth` (`self.Widget_HealthBar`) (`self.health`) (`self.maxHealth`) self)
  (`KismetSystemLibrary.K2_SetTimer` null "ResetSprite" 1.0))

(event `Key|V`
  (params (Key :type "Key Structure"))
  ;[1 1 1] DebugChat
  (:`Pressed`
    (`/Engine/EditorBlueprintResources/StandardMacros.FlipFlop`
      (:`A`
        (`/Game/Utilities/Librairies/BFL_Main.VisibilityDebugChat` "Visible"))
      (:`B`
        (`/Game/Utilities/Librairies/BFL_Main.VisibilityDebugChat` "Hidden")))))

(fn `AddBlockDamage`
  (params (blockCount :type Integer))
  (set `self.blockDamageStorage` (+ (`self.blockDamageStorage`) blockCount)))

(fn `AddManaEndTurn`
  (if (== (`self.mana`) 0)
    (if (!= (`self.manaMalus`) 0)
      (set `self.mana` (- 5 (`self.manaMalus`)))
      (set `self.manaMalus` 0)
      (return)
      (else
        (set `self.mana` 5)
        (return)))
    (elif (!= (`self.manaMalus`) 0)
      (set `self.mana` (- 6 (`self.manaMalus`)))
      (set `self.manaMalus` 0)
      (return)
      (else
        (set `self.mana` 6)
        (return)))))

(fn `Attack`
  (params (attackDamage :type "Float (double-precision)") (manaToRemove :type Integer))
  (returns (`isValid?` :type Boolean))
  (bind _enemyreference (`/Game/Systems/CardCombatSystem/CardCombat/Player/BP_CardController.enemyReference` (cast `/Game/Systems/CardCombatSystem/CardCombat/Player/BP_CardController` (`GameplayStatics.GetPlayerController` 0) :!pure true)))
  (`self.SetSprite` "/Game/Systems/CardCombatSystem/CardCombat/Img/CA_Art_Sprite_miaattack_Sprite.CA_Art_Sprite_miaattack_Sprite")
  (if (!= _enemyreference null)
    (`self.DealDamage` (`/Game/Systems/CardCombatSystem/CardCombat/BP_Entity.Widget_FeedbackDamage` _enemyreference) attackDamage _enemyreference self)
    (`KismetSystemLibrary.K2_SetTimer` null "ResetSprite" 1.0)
    (`self.RemoveMana` manaToRemove)
    (return true)))

(fn `Block`
  (params (blockDamage :type Integer) (manaToRemove :type Integer) (`increaseBlock?` :type Boolean))
  (returns (`isValid?` :type Boolean))
  (if (not (`self.AvoidAttack?`))
    (if `increaseBlock?`
      (`self.AddBlockDamage` (+ blockDamage (`self.increaseStats`)))
      (else
        (`self.AddBlockDamage` blockDamage)))
    (set `self.BlockDamage?` true)
    (`self.SetSprite` "/Game/Systems/CardCombatSystem/CardCombat/Img/CA_Art_Sprite_mianeutral_Sprite.CA_Art_Sprite_mianeutral_Sprite")
    (`self.RemoveMana` manaToRemove)
    (return true)
    (else
      (return false))))

(fn `BlockDamage`
  (params (Damage :type "Float (double-precision)") (Block :type "Float (double-precision)"))
  (returns (finalDamage :type "Float (double-precision)") (finalBlock :type "Float (double-precision)"))
  (bind _returnvalue (- Damage Block))
  (bind _returnvalue_2 (- Block (- (+ Damage Block) Block)))
  (if (< _returnvalue_2 0.0)
    (return _returnvalue 0.0)
    (else
      (return _returnvalue _returnvalue_2))))

(fn `CarefulBet`
  (params (min :type Integer) (max :type Integer) (manaToRemove :type Integer))
  (returns (`isValid?` :type Boolean))
  (if (not (`self.AvoidAttack?`))
    (`self.AddBlockDamage` (`KismetMathLibrary.RandomIntegerInRange` min max))
    (set `self.BlockDamage?` true)
    (`self.RemoveMana` manaToRemove)
    (return true)
    (else
      (return false))))

(fn `CheckMana`
  (params (numberToRemove :type Integer))
  (returns (`isRemove?` :type Boolean))
  (if (<= numberToRemove (`self.mana`))
    (return true)
    (else
      (return false))))

(fn `Dodge`
  (params (manaToRemove :type Integer))
  (returns (`isValid?` :type Boolean))
  (if (and (not (`self.BlockDamage?`)) (not (`self.AvoidAttack?`)))
    (set `self.AvoidAttack?` true)
    (`self.RemoveMana` manaToRemove)
    (return true)
    (else
      (return false))))

(fn `Gambler`
  (params (minDamage :type "Float (double-precision)") (maxDamage :type "Float (double-precision)") (manaToRemove :type Integer))
  (returns (`isValid?` :type Boolean))
  (`self.SetSprite` "/Game/Systems/CardCombatSystem/CardCombat/Img/CA_Art_Sprite_miahurt_Sprite.CA_Art_Sprite_miahurt_Sprite")
  (`self.DealDamage` (`self.Widget_FeedbackDamage`) (`KismetMathLibrary.Conv_IntToDouble` (`KismetMathLibrary.Round` (`KismetMathLibrary.RandomFloatInRange` minDamage maxDamage))) self self)
  (`KismetSystemLibrary.K2_SetTimer` null "ResetSprite" 1.0)
  (`self.RemoveMana` manaToRemove)
  (return true))

(fn `HolyTouch`
  (params (manaToRemove :type Integer))
  (returns (`isValid?` :type Boolean))
  (bind _asbp_card_game_mode (`/Game/Systems/CardCombatSystem/CardCombat/Cards/Libraries/BFL_Cards.Get Card Gamemode`))
  (bind _enemyreference (`/Game/Systems/CardCombatSystem/CardCombat/Player/BP_CardController.enemyReference` (cast `/Game/Systems/CardCombatSystem/CardCombat/Player/BP_CardController` (`GameplayStatics.GetPlayerController` 0) :!pure true)))
  (if (!= _enemyreference null)
    (`self.SetSprite` "/Game/Systems/CardCombatSystem/CardCombat/Img/CA_Art_Sprite_miaattack_Sprite.CA_Art_Sprite_miaattack_Sprite")
    (`/Game/Systems/CardCombatSystem/CardCombat/Player/BP_CardGameMode.DrawCards` _asbp_card_game_mode)
    (`self.DealDamage` (`/Game/Systems/CardCombatSystem/CardCombat/BP_Entity.Widget_FeedbackDamage` _enemyreference) (`KismetMathLibrary.Conv_IntToDouble` (* (- (`KismetArrayLibrary.Array_Length` (`/Game/Systems/CardCombatSystem/CardCombat/Cards/Widgets/WBP_CardHand.CardWidgetRef` (`/Game/Systems/CardCombatSystem/CardCombat/Cards/Widgets/WBP_CardCombatHUD.W_CardHand` (`/Game/Systems/CardCombatSystem/CardCombat/Player/BP_CardGameMode.WBP_CombatHUD_Reference` _asbp_card_game_mode)))) 1) 2)) _enemyreference self)
    (`KismetSystemLibrary.K2_SetTimer` null "ResetSprite" 1.0)
    (`self.RemoveMana` manaToRemove)
    (return true)))

(fn `Hysteria`
  (params (baseDamage :type "Float (double-precision)") (manaToRemove :type Integer))
  (returns (`isValid?` :type Boolean))
  (bind _enemyreference (`/Game/Systems/CardCombatSystem/CardCombat/Player/BP_CardController.enemyReference` (cast `/Game/Systems/CardCombatSystem/CardCombat/Player/BP_CardController` (`GameplayStatics.GetPlayerController` 0) :!pure true)))
  (if (!= _enemyreference null)
    (`self.SetSprite` "/Game/Systems/CardCombatSystem/CardCombat/Img/CA_Art_Sprite_miaattack_Sprite.CA_Art_Sprite_miaattack_Sprite")
    (`self.DealDamage` (`/Game/Systems/CardCombatSystem/CardCombat/BP_Entity.Widget_FeedbackDamage` _enemyreference) baseDamage _enemyreference self)
    (`/Game/Systems/CardCombatSystem/CardCombat/Cards/Libraries/BFL_Cards.ResetAdditionalDamage` "NewEnumerator0")
    (`KismetSystemLibrary.K2_SetTimer` null "ResetSprite" 1.0)
    (`self.RemoveMana` manaToRemove)
    (return true)))

(fn `Increase Stats`
  (params (amount :type "Float (double-precision)"))
  (set `self.increaseStats` (+ (`self.increaseStats`) amount)))

(fn `Inspiration`
  (params (manaToRemove :type Integer))
  (returns (`isValid?` :type Boolean))
  (bind _returnvalue (`|CreateWidget` "/Game/Systems/CardCombatSystem/CardCombat/Cards/Widgets/WBP_Inspiration.WBP_Inspiration_C"))
  (`UserWidget.AddToViewport` _returnvalue 0)
  (`self.RemoveMana` manaToRemove)
  (return true))

(fn `Investment`
  (params (BaseDamage :type "Float (double-precision)") (ManaToRemove :type Integer))
  (returns (`isValid?` :type Boolean))
  (bind _enemyreference (`/Game/Systems/CardCombatSystem/CardCombat/Player/BP_CardController.enemyReference` (cast `/Game/Systems/CardCombatSystem/CardCombat/Player/BP_CardController` (`GameplayStatics.GetPlayerController` 0) :!pure true)))
  (if (!= _enemyreference null)
    (`self.SetSprite` "/Game/Systems/CardCombatSystem/CardCombat/Img/CA_Art_Sprite_miaattack_Sprite.CA_Art_Sprite_miaattack_Sprite")
    (`self.DealDamage` (`/Game/Systems/CardCombatSystem/CardCombat/BP_Entity.Widget_FeedbackDamage` _enemyreference) (+ BaseDamage (`self.increaseStats`)) _enemyreference self)
    (`KismetSystemLibrary.K2_SetTimer` null "ResetSprite" 1.0)
    (`self.RemoveMana` ManaToRemove)
    (return true)))

(fn `Recognition`
  (params (manaToRemove :type Integer))
  (returns (`isValid?` :type Boolean))
  (set `self.takingDamageEndTurn` (`KismetMathLibrary.Conv_IntToDouble` (`/Game/Systems/CardCombatSystem/CardCombat/Player/BP_CardGameMode.roundNumber` (`/Game/Systems/CardCombatSystem/CardCombat/Cards/Libraries/BFL_Cards.Get Card Gamemode`))))
  (`self.RemoveMana` manaToRemove)
  (return true))

(fn `RemoveMana`
  (params (numberToRemove :type Integer))
  (set `self.mana` (- (`self.mana`) numberToRemove)))

(fn `ResetBlockDamage`
  (set `self.BlockDamage?` false)
  (set `self.blockDamageStorage` 0))

(fn `ResetSprite`
  (`self.SetSprite` "/Game/Systems/CardCombatSystem/CardCombat/Img/CA_Art_Sprite_mianeutral_Sprite.CA_Art_Sprite_mianeutral_Sprite"))

(fn `ResetStats`
  (set `self.increaseStats` 0.0))

(fn `ReshuffleCards`
  (locals (columnName :type Name) (cardCount :type Integer))
  (`self.SetupCards`)
  (if (not (`KismetArrayLibrary.Array_IsEmpty` (`/Game/Systems/CardCombatSystem/CardCombat/Cards/Widgets/WBP_CardHand.CardWidgetRef` (`/Game/Systems/CardCombatSystem/CardCombat/Cards/Widgets/WBP_CardCombatHUD.W_CardHand` (`/Game/Systems/CardCombatSystem/CardCombat/Player/BP_CardGameMode.WBP_CombatHUD_Reference` (`/Game/Systems/CardCombatSystem/CardCombat/Cards/Libraries/BFL_Cards.Get Card Gamemode`))))))
    (for _array_element (`/Game/Systems/CardCombatSystem/CardCombat/Cards/Widgets/WBP_CardHand.CardWidgetRef` (`/Game/Systems/CardCombatSystem/CardCombat/Cards/Widgets/WBP_CardCombatHUD.W_CardHand` (`/Game/Systems/CardCombatSystem/CardCombat/Player/BP_CardGameMode.WBP_CombatHUD_Reference` (`/Game/Systems/CardCombatSystem/CardCombat/Cards/Libraries/BFL_Cards.Get Card Gamemode`))))
      (bind _returnvalue (`KismetStringLibrary.Conv_StringToName` (`KismetTextLibrary.Conv_TextToString` (`.CardName_2_700057764056FABB48B2B1BECCF8903D` (break `/Game/Systems/CardCombatSystem/CardCombat/Cards/Structure/S_CardInfo` (`/Game/Systems/CardCombatSystem/CardCombat/Cards/Widgets/WBP_Cards.CardInfo` _array_element))))))
      (bind _value (`BlueprintMapLibrary.Map_Find` (`self.cards`) _returnvalue))
      (`BlueprintMapLibrary.Map_Add` (`self.cards`) _returnvalue (- _value 1))
      (if (== _value 0)
        (`BlueprintMapLibrary.Map_Remove` (`self.cards`) _returnvalue)))))

(fn `RollOfTheDice`
  (params (addtionalDamage :type "Float (double-precision)") (manaToRemove :type Integer))
  (returns (`isValid?` :type Boolean))
  (bind _enemyreference (`/Game/Systems/CardCombatSystem/CardCombat/Player/BP_CardController.enemyReference` (cast `/Game/Systems/CardCombatSystem/CardCombat/Player/BP_CardController` (`GameplayStatics.GetPlayerController` 0) :!pure true)))
  (if (!= _enemyreference null)
    (`self.SetSprite` "/Game/Systems/CardCombatSystem/CardCombat/Img/CA_Art_Sprite_miaattack_Sprite.CA_Art_Sprite_miaattack_Sprite")
    ;[1 1 1] Damage Enemy
    (`self.DealDamage` (`/Game/Systems/CardCombatSystem/CardCombat/BP_Entity.Widget_FeedbackDamage` _enemyreference) (+ (`KismetMathLibrary.Conv_IntToDouble` (`KismetMathLibrary.RandomIntegerInRange` 10 16)) addtionalDamage) _enemyreference self)
    ;[1 1 1] Damage Player
    (`self.DealDamage` (`self.Widget_FeedbackDamage`) (`KismetMathLibrary.Conv_IntToDouble` (`KismetMathLibrary.RandomIntegerInRange` 2 6)) self _enemyreference)
    (`KismetSystemLibrary.K2_SetTimer` null "ResetSprite" 1.0)
    (`self.RemoveMana` manaToRemove)
    (return true)))

(fn `SetSprite`
  (params (NewSprite :type "PaperSprite Object Reference"))
  (`PaperSpriteComponent.SetSprite` (`self.PaperSprite`) NewSprite))

(fn `SetupCards`
  (bind _outrownames (`DataTableFunctionLibrary.GetDataTableRowNames` "/Game/Systems/CardCombatSystem/CardCombat/Cards/Datatable/DT_Cards.DT_Cards"))
  (for _array_element _outrownames
    (bind _returnvalue (`|GetDataTableRow` "/Game/Systems/CardCombatSystem/CardCombat/Cards/Datatable/DT_Cards.DT_Cards" _array_element)
      (:`then`
        (bind (_cardid _cardname _image _carddescription _backgroundcolor _mana _type _cardnumber _archetype _isautoplayed_ _isplayedendturn_ _cardtier _cardstatut) (break `/Game/Systems/CardCombatSystem/CardCombat/Cards/Structure/S_CardInfo` _returnvalue))
        (if (`|EnumEquality` _cardstatut "NewEnumerator2")
          (`BlueprintMapLibrary.Map_Add` (`self.cards`) _array_element _cardnumber)
          (else
            (bind _value (`BlueprintMapLibrary.Map_Find` (`/Game/Utilities/GameInstance/GameInstance_Tomebound.affinityBar` (`/Game/Utilities/Librairies/BFL_Main.GetGameInstanceTomebound`)) _archetype))
            (if (!= _value 0)
              (if (< _value 0)
                (if (and (>= _cardtier _value) (`|EnumEquality` _cardstatut "NewEnumerator0"))
                  (`BlueprintMapLibrary.Map_Add` (`self.cards`) _array_element 1))
                (elif (and (<= _cardtier _value) (`|EnumEquality` _cardstatut "NewEnumerator1"))
                  (`BlueprintMapLibrary.Map_Add` (`self.cards`) _array_element 2))))))))))

(fn `Spell`
  (params (manaToRemove :type Integer) (spellDamage :type "Float (double-precision)") (manaMalus :type Integer))
  (returns (`isValid?` :type Boolean))
  (bind _enemyreference (`/Game/Systems/CardCombatSystem/CardCombat/Player/BP_CardController.enemyReference` (cast `/Game/Systems/CardCombatSystem/CardCombat/Player/BP_CardController` (`GameplayStatics.GetPlayerController` 0) :!pure true)))
  (if (!= _enemyreference null)
    (`self.DealDamage` (`/Game/Systems/CardCombatSystem/CardCombat/BP_Entity.Widget_FeedbackDamage` _enemyreference) spellDamage _enemyreference self)
    (`self.RemoveMana` manaToRemove)
    (set `self.manaMalus` (+ (`self.manaMalus`) manaMalus))
    (return true)))

(fn `TakeDamagePlayerEndTurn`
  (`self.DealDamage` (`self.Widget_FeedbackDamage`) (`self.takingDamageEndTurn`))
  (set `self.takingDamageEndTurn` 0.0))

(fn `UserConstructionScript`)