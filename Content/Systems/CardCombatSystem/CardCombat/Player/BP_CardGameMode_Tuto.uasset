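; Tutorial variant of the card combat game mode, which starts a card game with a preset hand and a tutorial UI.
; On BeginPlay it sets TutorialMode before running the parent logic, then creates the WBP_Tuto widget and adds it to the viewport.
; After a short delay it replaces the card player's Cards with the TutorialHand.
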(event `self.ReceiveBeginPlay`
  (set `self.tutorialMode` true)
  (`parent.ReceiveBeginPlay`)
  (bind _returnvalue (`|CreateWidget` "/Game/Systems/CardCombatSystem/CardCombat/Widgets/WBP_Tuto.WBP_Tuto_C"))
  (bind _output_get (set `self.UITutoRef` _returnvalue))
  (`UserWidget.AddToViewport` _output_get 0)
  (`KismetSystemLibrary.Delay` 1.0)
  (set `/Game/Systems/CardCombatSystem/CardCombat/Player/BP_Card_Player.cards` (`self.tutorialHand`) (`/Game/Systems/CardCombatSystem/CardCombat/Cards/Libraries/BFL_Cards.GetCardPlayer`)))

(fn `UserConstructionScript`
  (`parent.UserConstructionScript`))