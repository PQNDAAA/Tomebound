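; Player controller for the card combat system that lets the player click to select an enemy as the current target.
; A left click traces under the cursor for a BP_Enemy and acts only during the first turn state of the card game mode.
; It stores the enemy and shows its selection arrow; clicking that enemy again deselects it.
; Other enemies are ignored while a valid selection exists.
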(event `Key|LeftMouseButton`
  (params (Key :type "Key Structure"))
  (bind _enemyreference (`self.enemyReference`))
  (bind _selectionarrow (`/Game/Systems/CardCombatSystem/CardCombat/AI/Character/BP/BP_Enemy.SelectionArrow` _enemyreference))
  (:`Pressed`
    (bind _asbp_enemy (cast `/Game/Systems/CardCombatSystem/CardCombat/AI/Character/BP/BP_Enemy` (`.HitActor` (`GameplayStatics.BreakHitResult` (`self.GetHitResultUnderCursorByChannel` "TraceTypeQuery1")))))
    (if (`|EnumEquality` (`/Game/Systems/CardCombatSystem/CardCombat/Player/BP_CardGameMode.enum_Turn` (`/Game/Systems/CardCombatSystem/CardCombat/Cards/Libraries/BFL_Cards.Get Card Gamemode`)) "NewEnumerator0")
      (if (not (`self.hasClickedOnEnemy?`))
        (set `self.enemyReference` _asbp_enemy :!label _label)
        (set `self.hasClickedOnEnemy?` true)
        (`SceneComponent.SetHiddenInGame` _selectionarrow false false)
        (else
          (`/Engine/EditorBlueprintResources/StandardMacros.IsValid` _enemyreference
            (:`Is Valid`
              (if (== _enemyreference _asbp_enemy)
                (set `self.hasClickedOnEnemy?` false)
                (`SceneComponent.SetHiddenInGame` _selectionarrow true false)
                (set `self.enemyReference` null)))
            (:`Is Not Valid`
              (goto _label))))))))

(fn `UserConstructionScript`)