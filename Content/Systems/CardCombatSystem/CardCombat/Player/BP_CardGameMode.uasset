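; Game mode for the card combat system that creates the combat HUD and runs the turn loop between player and enemy.
; An EnumTurn state drives TurnCombat: player turns count rounds and refill the hand, while enemy turns only wait before switching back.
; SwitchTurn applies end-of-turn player effects, auto-played cards and ID-matched hand bonuses, or resets block and dodge after enemy turns.
; An invalid player switches to EndGame, which is an empty stub.
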(event `self.ReceiveBeginPlay`
  (bind _returnvalue (`|CreateWidget` "/Game/Systems/CardCombatSystem/CardCombat/Cards/Widgets/WBP_CardCombatHUD.WBP_CardCombatHUD_C" null (`self.maxCardCount`)))
  (bind _output_get (set `self.WBP_CombatHUD_Reference` _returnvalue))
  (`UserWidget.AddToViewport` _output_get 0)
  (set `PlayerController.bShowMouseCursor` true (`GameplayStatics.GetPlayerController` 0))
  (set `self.currentLevelIndex` 0)
  (`self.StartGame`))

(event `StartGame`
  (bind _asbp_card_player (`/Game/Systems/CardCombatSystem/CardCombat/Cards/Libraries/BFL_Cards.GetCardPlayer`))
  ;[1 1 1] StartGame
  (`/Engine/EditorBlueprintResources/StandardMacros.IsValid` _asbp_card_player
    (:`Is Valid`
      (`/Game/Systems/CardCombatSystem/CardCombat/Player/BP_Card_Player.SetupCards` _asbp_card_player))
    (:`Is Not Valid`
      (set `self.enum_Turn` "NewEnumerator2")))
  (`self.TurnCombat`))

(event `TurnCombat`
  ;[1 1 1] Combat Loop
  (switch `/Game/Systems/CardCombatSystem/CardCombat/Enumeration/E_Turn` (`self.enum_Turn`)
    (:`NewEnumerator0`
      (`self.playerTurn`))
    (:`NewEnumerator1`
      (`self.enemyTurn`))
    (:`NewEnumerator2`
      (`self.EndGame`))))

(event `playerTurn`
  ;[1 1 1] Player Turn
  (`KismetSystemLibrary.Delay` 0.2)
  (`self.AddRound`)
  (`self.CheckCardPlayer`)
  (set `/Game/Systems/CardCombatSystem/CardCombat/Widgets/WBP_Turn.turnText` "YOUR TURN" (`/Game/Systems/CardCombatSystem/CardCombat/Cards/Widgets/WBP_CardCombatHUD.WBP_Turn` (`self.WBP_CombatHUD_Reference`))))

(event `enemyTurn`
  ;[1 1 1] Enemy Turn
  (set `/Game/Systems/CardCombatSystem/CardCombat/Widgets/WBP_Turn.turnText` "ENEMY TURN" (`/Game/Systems/CardCombatSystem/CardCombat/Cards/Widgets/WBP_CardCombatHUD.WBP_Turn` (`self.WBP_CombatHUD_Reference`)))
  (`KismetSystemLibrary.Delay` 0.75)
  (`self.SwitchTurn`)
  (`self.TurnCombat`))

(fn `AddBlockDodge`
  (params (cardID :type Integer) (cards :type "Array of /Game/Systems/CardCombatSystem/CardCombat/Cards/Widgets/WBP_Cards Object Reference"))
  (bind _asbp_card_player (`/Game/Systems/CardCombatSystem/CardCombat/Cards/Libraries/BFL_Cards.GetCardPlayer`))
  (bind _cardsl (`self.GetHandCardByID` cardID cards))
  (if (`KismetArrayLibrary.Array_IsNotEmpty` _cardsl)
    (for _ _cardsl
      (`/Engine/EditorBlueprintResources/StandardMacros.IsValid` _asbp_card_player
        (:`Is Valid`
          (`/Game/Systems/CardCombatSystem/CardCombat/Player/BP_Card_Player.AddBlockDamage` _asbp_card_player 2))))))

(fn `AddRound`
  (set `self.roundNumber` (+ (`self.roundNumber`) 1)))

(fn `CheckCardPlayer`
  (locals (cardHandLength :type Integer :default 0))
  (bind _cardwidgetref (`/Game/Systems/CardCombatSystem/CardCombat/Cards/Widgets/WBP_CardHand.CardWidgetRef` (`/Game/Systems/CardCombatSystem/CardCombat/Cards/Widgets/WBP_CardCombatHUD.W_CardHand` (`self.WBP_CombatHUD_Reference`))))
  (bind _returnvalue (`KismetArrayLibrary.Array_Length` _cardwidgetref))
  (set `local.cardHandLength` _returnvalue)
  (if (< _returnvalue (`self.maxCardCount`))
    (for _ (range (+ (- (`self.maxCardCount`) (`local.cardHandLength`) 1) 1))
      (`self.DrawCards`)))
  (`self.SetAdditionalDamage` "NewEnumerator0" _cardwidgetref 11))

(fn `CheckCardPlayerEndTurn`
  (params (cards :type "Array of /Game/Systems/CardCombatSystem/CardCombat/Cards/Widgets/WBP_Cards Object Reference"))
  (for _array_element cards
    (if (`.isPlayedEndTurn?_44_EFE306FA4B1E31F086472986676A8D43` (break `/Game/Systems/CardCombatSystem/CardCombat/Cards/Structure/S_CardInfo` (`/Game/Systems/CardCombatSystem/CardCombat/Cards/Widgets/WBP_Cards.CardInfo` _array_element)))
      (`/Engine/EditorBlueprintResources/StandardMacros.IsValid` (`/Game/Systems/CardCombatSystem/CardCombat/Cards/Libraries/BFL_Cards.GetCardPlayer`)
        (:`Is Valid`
          (`/Game/Systems/CardCombatSystem/CardCombat/Cards/BlueprintType/BP_CardBase.CardOnClicked` (`/Game/Systems/CardCombatSystem/CardCombat/Cards/Widgets/WBP_Cards.CardBase` _array_element)))
        (:`Is Not Valid`
          (break))))))

(fn `DrawCards`
  (bind _w_cardhand (`/Game/Systems/CardCombatSystem/CardCombat/Cards/Widgets/WBP_CardCombatHUD.W_CardHand` (`self.WBP_CombatHUD_Reference`)))
  (bind (_out_row _isempty_) (`/Game/Systems/CardCombatSystem/CardCombat/Cards/Libraries/BFL_Cards.GetAvailaibleCards`))
  (if (not _isempty_)
    (message `/Game/Systems/CardCombatSystem/CardCombat/Cards/Interface/BI_AddCard.AddCard` _w_cardhand _out_row _isempty_)
    (else
      (message `/Game/Systems/CardCombatSystem/CardCombat/Cards/Interface/BI_AddCard.AddCard` _w_cardhand _out_row _isempty_)
      (`/Game/Systems/CardCombatSystem/CardCombat/Player/BP_Card_Player.ReshuffleCards` (`/Game/Systems/CardCombatSystem/CardCombat/Cards/Libraries/BFL_Cards.GetCardPlayer`)))))

(fn `EndGame`)

(fn `GetHandCardByID`
  (params (cardID :type Integer) (cards :type "Array of /Game/Systems/CardCombatSystem/CardCombat/Cards/Widgets/WBP_Cards Object Reference"))
  (returns (cardsL :type "Array of /Game/Systems/CardCombatSystem/CardCombat/Cards/Widgets/WBP_Cards Object Reference"))
  (locals (cardsList :type "Array of /Game/Systems/CardCombatSystem/CardCombat/Cards/Widgets/WBP_Cards Object Reference"))
  (for _array_element cards
    (if (== cardID (`.cardID_47_1C4896E44D1BC2162F194AAF2693E4E5` (break `/Game/Systems/CardCombatSystem/CardCombat/Cards/Structure/S_CardInfo` (`/Game/Systems/CardCombatSystem/CardCombat/Cards/Widgets/WBP_Cards.CardInfo` _array_element))))
      (`KismetSystemLibrary.PrintString` (`KismetSystemLibrary.GetDisplayName` _array_element))
      (`KismetArrayLibrary.Array_AddUnique` (`local.cardsList`) _array_element)))
  (return (`local.cardsList`)))

(fn `SetAdditionalDamage`
  (params (cardType :type "/Game/Systems/CardCombatSystem/CardCombat/Cards/BlueprintType/Enum/E_CardType Enum" :default "NewEnumerator0") (cards :type "Array of /Game/Systems/CardCombatSystem/CardCombat/Cards/Widgets/WBP_Cards Object Reference (by ref)") (cardID :type Integer))
  (bind _cardsl (`self.GetHandCardByID` cardID cards))
  (if (`KismetArrayLibrary.Array_IsNotEmpty` _cardsl)
    (for _array_element _cardsl
      (bind _outactors (`GameplayStatics.GetAllActorsOfClass` "/Game/Systems/CardCombatSystem/CardCombat/Cards/BlueprintType/BP_CardBase.BP_CardBase_C"))
      (for _array_element_2 _outactors
        (if (`|EnumEquality` cardType (`/Game/Systems/CardCombatSystem/CardCombat/Cards/BlueprintType/BP_CardBase.cardType` _array_element_2))
          (set `/Game/Systems/CardCombatSystem/CardCombat/Cards/BlueprintType/BP_CardBase.addtionalDamage` (+ (`/Game/Systems/CardCombatSystem/CardCombat/Cards/BlueprintType/BP_CardBase.addtionalDamage` _array_element_2) (`/Game/Systems/CardCombatSystem/CardCombat/Cards/BlueprintType/BP_Hysteria.baseAdditionalDamage` (cast `/Game/Systems/CardCombatSystem/CardCombat/Cards/BlueprintType/BP_Hysteria` (`/Game/Systems/CardCombatSystem/CardCombat/Cards/Widgets/WBP_Cards.CardBase` _array_element) :!pure true))) _array_element_2))))))

(fn `SwitchTurn`
  (bind _asbp_card_player (`/Game/Systems/CardCombatSystem/CardCombat/Cards/Libraries/BFL_Cards.GetCardPlayer`))
  (bind _asbp_card_player_2 (`/Game/Systems/CardCombatSystem/CardCombat/Cards/Libraries/BFL_Cards.GetCardPlayer`))
  (bind _cardwidgetref (`/Game/Systems/CardCombatSystem/CardCombat/Cards/Widgets/WBP_CardHand.CardWidgetRef` (`/Game/Systems/CardCombatSystem/CardCombat/Cards/Widgets/WBP_CardCombatHUD.W_CardHand` (`self.WBP_CombatHUD_Reference`))))
  (if (`|EnumEquality` (`self.enum_Turn`) "NewEnumerator0")
    (set `/Game/Systems/CardCombatSystem/CardCombat/Player/BP_CardController.enemyReference` null (cast `/Game/Systems/CardCombatSystem/CardCombat/Player/BP_CardController` (`GameplayStatics.GetPlayerController` 0) :!pure true))
    (`/Engine/EditorBlueprintResources/StandardMacros.IsValid` _asbp_card_player
      (:`Is Valid`
        (`/Game/Systems/CardCombatSystem/CardCombat/Player/BP_Card_Player.AddManaEndTurn` _asbp_card_player)
        (`/Game/Systems/CardCombatSystem/CardCombat/Player/BP_Card_Player.TakeDamagePlayerEndTurn` _asbp_card_player)
        (`/Game/Systems/CardCombatSystem/CardCombat/Cards/Libraries/BFL_Cards.ResetAllAdditionalDamage` "NewEnumerator0")
        (`/Game/Systems/CardCombatSystem/CardCombat/Cards/Libraries/BFL_Cards.ResetAllMana`)
        (`/Engine/EditorBlueprintResources/StandardMacros.IsValid` _asbp_card_player
          (:`Is Valid`
            (`self.CheckCardPlayerEndTurn` _cardwidgetref)
            (`self.AddBlockDodge` 2 _cardwidgetref)
            (`/Engine/EditorBlueprintResources/StandardMacros.IsValid` (`/Game/Systems/CardCombatSystem/CardCombat/Cards/Libraries/BFL_Cards.GetCardPlayer`)
              (:`Is Valid`
                (set `self.enum_Turn` "NewEnumerator1"))
              (:`Is Not Valid`
                (set `self.enum_Turn` "NewEnumerator2"))))
          (:`Is Not Valid`
            (set `self.enum_Turn` "NewEnumerator2"))))
      (:`Is Not Valid`
        (set `self.enum_Turn` "NewEnumerator2")))
    (else
      (bind _outactors (`GameplayStatics.GetAllActorsOfClass` "/Game/Systems/CardCombatSystem/CardCombat/AI/Character/BP/BP_Enemy.BP_Enemy_C"))
      (for _array_element _outactors
        (set `/Game/Systems/CardCombatSystem/CardCombat/AI/Character/BP/BP_Enemy.enemyBlockDamage` false _array_element))
      (`/Engine/EditorBlueprintResources/StandardMacros.IsValid` _asbp_card_player_2
        (:`Is Valid`
          (`/Game/Systems/CardCombatSystem/CardCombat/Player/BP_Card_Player.ResetBlockDamage` _asbp_card_player_2)
          (set `/Game/Systems/CardCombatSystem/CardCombat/Player/BP_Card_Player.AvoidAttack?` false _asbp_card_player_2)
          (set `self.enum_Turn` "NewEnumerator0"))
        (:`Is Not Valid`
          (set `self.enum_Turn` "NewEnumerator2"))))))

(fn `UserConstructionScript`)