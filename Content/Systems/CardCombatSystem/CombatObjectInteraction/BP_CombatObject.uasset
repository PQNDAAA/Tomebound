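; Interactable combat object that shows a dialog and then loads the level named by LevelName to start a fight.
; ObjectInteraction calls its parent, disables pawn input, creates WBP_ObjectDialog with DialogText, then CheckWidget polls until the dialog block hides and opens the level.
; Box overlap gates a left-click cursor trace for the CombatObject tag, but that check leads nowhere and its old dialog logic is disconnected.
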(event `Key|LeftMouseButton`
  (params (Key :type "Key Structure"))
  ;[1 1 1] Left Mouse Button Event on Overlap
  ;;[1 1 1] Check Mouse Cursor
  (:`Pressed`
    (`/Engine/EditorBlueprintResources/StandardMacros.Gate` true :!label _label
      (:`Exit`
        (if (and (`self.ActorHasTag` (`.HitActor` (`GameplayStatics.BreakHitResult` (`PlayerController.GetHitResultUnderCursorByChannel` (`GameplayStatics.GetPlayerController` 0) "TraceTypeQuery1" true))) "CombatObject") (not (`KismetSystemLibrary.IsValid` (`self.WBP_ObjectDialogReference`))))
          _)))))

(event `self.Box.OnComponentBeginOverlap`
  (params (OverlappedComponent :type "PrimitiveComponent Object Reference") (OtherActor :type "Actor Object Reference") (OtherComp :type "PrimitiveComponent Object Reference") (OtherBodyIndex :type Integer) (bFromSweep :type Boolean) (SweepResult :type "HitResult Structure (by ref)"))
  ;[1 1 1] Left Mouse Button Event on Overlap
  (`self.EnableInput` (`GameplayStatics.GetPlayerController` 0))
  (goto _label :!via `Open`))

(event `self.Box.OnComponentEndOverlap`
  (params (OverlappedComponent :type "PrimitiveComponent Object Reference") (OtherActor :type "Actor Object Reference") (OtherComp :type "PrimitiveComponent Object Reference") (OtherBodyIndex :type Integer))
  ;[1 1 1] Left Mouse Button Event on Overlap
  (`self.DisableInput` (`GameplayStatics.GetPlayerController` 0))
  (goto _label :!via `Close`))

(event `CheckWidget`
  ;[1 1 1] Check Widget to start the fight
  (`KismetSystemLibrary.Delay` 0.2)
  (if (`Widget.IsVisible` (`/Game/Widgets/WBP_ObjectDialog.DialogBlock` (`self.WBP_ObjectDialogReference`)))
    (`self.CheckWidget`)
    (else
      (set `self.WBP_ObjectDialogReference` null)
      (`GameplayStatics.OpenLevel` (`self.Level Name`)))))

(fn `ObjectInteraction`
  (`parent.ObjectInteraction`)
  (`self.DisableInput` (`GameplayStatics.GetPlayerPawn` 0) (`GameplayStatics.GetPlayerController` 0))
  (bind _returnvalue (`|CreateWidget` "/Game/Widgets/WBP_ObjectDialog.WBP_ObjectDialog_C" null null))
  (bind _output_get (set `self.WBP_ObjectDialogReference` _returnvalue))
  (`UserWidget.AddToViewport` _output_get 0)
  (`/Game/Utilities/Librairies/BFL_Main.SetDialogBlockOnWidget` (`/Game/Widgets/WBP_ObjectDialog.DialogBlock` (`self.WBP_ObjectDialogReference`)) (`self.dialogText`))
  (`self.CheckWidget`))

(fn `UserConstructionScript`)