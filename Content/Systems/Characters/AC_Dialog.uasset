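; Dialog component that runs event-keyed character conversations in a WBP_CharacterDialog widget, disabling player pawn input while open.
; A Dialog/Choice/Finished state drives progression: each step increments an index to look up text in DT_Dialog and the speaker's image and name in DT_CharacterDialog.
; When no line matches, it offers the event's DT_Choice entry, or closes if none exists.
; Closing resets the index, but the state reset to Dialog is unconnected.
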(event `self.ReceiveBeginPlay`)

(fn `AddChoice`
  (params (choiceStructure :type "/Game/Systems/Characters/Structure/S_Choice Structure (by ref)"))
  (`/Game/Systems/Characters/Widgets/WBP_CharacterDialog.CreateChoice` (`self.dialogWidgetReference`) choiceStructure))

(fn `AddDialog`
  (params (targetCharacterDialog :type "/Game/Systems/Characters/BP/BP_Character Class Reference") (text :type Text))
  (`/Game/Systems/Characters/Widgets/WBP_CharacterDialog.SetCurrentDialogText` (`self.dialogWidgetReference`) text)
  (`self.UpdateCharacterImage` targetCharacterDialog))

(fn `AddDialogIndex`
  (params (addNumber :type Integer))
  (set `self.dialogIndex` (+ (`self.dialogIndex`) addNumber)))

(fn `CloseDialog`
  (`self.ResetDialogIndex`)
  (`Actor.EnableInput` (`GameplayStatics.GetPlayerPawn` 0) (`GameplayStatics.GetPlayerController` 0))
  (`Widget.RemoveFromParent` (`self.dialogWidgetReference`)))

(fn `OpenDialog`
  (params (currentEvent :type "/Game/Systems/Characters/Enum/Enum_Events Enum" :default "NewEnumerator1"))
  (set `self.current Event` currentEvent)
  (`Actor.DisableInput` (`GameplayStatics.GetPlayerPawn` 0) (`GameplayStatics.GetPlayerController` 0))
  (bind _returnvalue (`|CreateWidget` "/Game/Systems/Characters/Widgets/WBP_CharacterDialog.WBP_CharacterDialog_C" null self))
  (bind _output_get (set `self.dialogWidgetReference` _returnvalue))
  (`UserWidget.AddToViewport` _output_get 0)
  (`self.ProgressDialog`))

(fn `ProgressDialog`
  (switch `/Game/Systems/Characters/Enum/E_DialogState` (`self.currentState`)
    (:`NewEnumerator0`
      (`self.AddDialogIndex` 1)
      (`self.UpdateDialog`))
    (:`NewEnumerator1`
      (`self.CloseDialog`))))

(fn `ResetDialogIndex`
  (set `self.dialogIndex` 0))

(fn `SearchChoice`
  (returns (`Out Row` :type "/Game/Systems/Characters/Structure/S_Choice Structure"))
  (bind _outrownames (`DataTableFunctionLibrary.GetDataTableRowNames` "/Game/Systems/Characters/Datatable/DT_Choice.DT_Choice"))
  (for _array_element _outrownames
    (bind _returnvalue (`|GetDataTableRow` "/Game/Systems/Characters/Datatable/DT_Choice.DT_Choice" _array_element)
      (:`then`
        (if (`|EnumEquality` (`self.current Event`) (`.eventName_2_C30C0C8C43080603F74D919C2076497B` (break `/Game/Systems/Characters/Structure/S_Choice` _returnvalue)))
          (return _returnvalue)))))
  (set `self.currentState` "NewEnumerator1")
  (return))

(fn `SearchDialog`
  (returns (targetCharacter :type "/Game/Systems/Characters/BP/BP_Character Class Reference") (currentText :type Text))
  (bind _outrownames (`DataTableFunctionLibrary.GetDataTableRowNames` "/Game/Systems/Characters/Datatable/DT_Dialog.DT_Dialog"))
  (for _array_element _outrownames
    (bind _returnvalue (`|GetDataTableRow` "/Game/Systems/Characters/Datatable/DT_Dialog.DT_Dialog" _array_element)
      (:`then`
        (bind (_eventname _targetcharacter _dialogtext) (break `/Game/Systems/Characters/Structure/S_Dialog` _returnvalue))
        (if (`|EnumEquality` (`self.current Event`) _eventname)
          (bind (_value _returnvalue_2) (`BlueprintMapLibrary.Map_Find` _dialogtext (`self.dialogIndex`)))
          (if _returnvalue_2
            (return _targetcharacter _value))))))
  (set `self.currentState` "NewEnumerator2")
  (return null ""))

(fn `UpdateCharacterImage`
  (params (targetCharacterDialog :type "/Game/Systems/Characters/BP/BP_Character Class Reference"))
  (locals (targetCharacter :type "/Game/Systems/Characters/BP/BP_Character Class Reference"))
  (set `local.targetCharacter` targetCharacterDialog)
  (bind _outrownames (`DataTableFunctionLibrary.GetDataTableRowNames` "/Game/Systems/Characters/Datatable/DT_CharacterDialog.DT_CharacterDialog"))
  (for _array_element _outrownames
    (bind _returnvalue (`|GetDataTableRow` "/Game/Systems/Characters/Datatable/DT_CharacterDialog.DT_CharacterDialog" _array_element)
      (:`then`
        (bind (_charactername _charactertype _blackimage _colorimage) (break `/Game/Systems/Characters/Structure/S_CharacterDialog` _returnvalue))
        (if (== _charactertype (`local.targetCharacter`))
          (`/Game/Systems/Characters/Widgets/WBP_CharacterDialog.SetCurrentCharacterImage` (`self.dialogWidgetReference`) _colorimage _charactername))))))

(fn `UpdateChoice`
  (bind _out_row (`self.SearchChoice`))
  (switch `/Game/Systems/Characters/Enum/E_DialogState` (`self.currentState`)
    (:`NewEnumerator1`
      (`self.CloseDialog`))
    (:`NewEnumerator2`
      (`self.AddChoice` _out_row))))

(fn `UpdateDialog`
  (bind (_targetcharacter _currenttext) (`self.SearchDialog`))
  (switch `/Game/Systems/Characters/Enum/E_DialogState` (`self.currentState`)
    (:`NewEnumerator0`
      (`self.AddDialog` _targetcharacter _currenttext))
    (:`NewEnumerator1`
      (`self.CloseDialog`))
    (:`NewEnumerator2`
      (`self.UpdateChoice`))))