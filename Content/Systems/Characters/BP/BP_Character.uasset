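; BP_Character is a talkable character that opens a dialog box when clicked while something overlaps its Box.
; At BeginPlay it scans DT_Dialog for rows matching its actor and Event, caching the dialog text array.
; Box overlaps toggle its input and a gate; a cursor trace on a "CharacterActor"-tagged component then disables pawn input and spawns WBP_CharacterDialog, one at a time.
; Helper functions set the floating name widget and clear the dialog reference.
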(event `self.ReceiveBeginPlay`
  ;[0.69 0 0] Update Character at Begin Play
  (`self.UpdateCharacter`))

(event `Key|LeftMouseButton`
  (params (Key :type "Key Structure"))
  (bind (_bblockinghit _binitialoverlap _time _distance _location _impactpoint _normal _impactnormal _physmat _hitactor _hitcomponent) (`GameplayStatics.BreakHitResult` (`PlayerController.GetHitResultUnderCursorByChannel` (`GameplayStatics.GetPlayerController` 0) "TraceTypeQuery1" true)))
  (:`Pressed`
    (`/Engine/EditorBlueprintResources/StandardMacros.IsValid` _hitcomponent
      (:`Is Valid`
        (if (and (`ActorComponent.ComponentHasTag` _hitcomponent "CharacterActor") (not (`KismetSystemLibrary.IsValid` (`self.dialogBox_Reference`))))
          (`/Engine/EditorBlueprintResources/StandardMacros.Gate` true :!label _label
            (:`Exit`
              (`self.DisableInput` (`GameplayStatics.GetPlayerPawn` 0) (`GameplayStatics.GetPlayerController` 0))
              (bind _returnvalue (`|CreateWidget` "/Game/Systems/Characters/Widgets/WBP_CharacterDialog.WBP_CharacterDialog_C" null self (`self.dialogTextArray`)))
              (bind _output_get (set `self.dialogBox_Reference` _returnvalue))
              (`UserWidget.AddToViewport` _output_get 0)
              (`/Game/Utilities/Librairies/BFL_Main.PrintDebugChat` (`|FormatText` "PlayerDialog" self) "PlayerDialog"))))))))

(event `self.Box.OnComponentBeginOverlap`
  (params (OverlappedComponent :type "PrimitiveComponent Object Reference") (OtherActor :type "Actor Object Reference") (OtherComp :type "PrimitiveComponent Object Reference") (OtherBodyIndex :type Integer) (bFromSweep :type Boolean) (SweepResult :type "HitResult Structure (by ref)"))
  (`self.EnableInput` (`GameplayStatics.GetPlayerController` 0))
  (goto _label :!via `Open`))

(event `self.Box.OnComponentEndOverlap`
  (params (OverlappedComponent :type "PrimitiveComponent Object Reference") (OtherActor :type "Actor Object Reference") (OtherComp :type "PrimitiveComponent Object Reference") (OtherBodyIndex :type Integer))
  (`self.DisableInput` (`GameplayStatics.GetPlayerController` 0))
  (goto _label :!via `Close`))

(fn `ResetDialogBox`
  (set `self.dialogBox_Reference` null))

(fn `SetActorNameOnWidget`
  (bind _aswbp_actor_name (cast `/Game/Widgets/WBP_ActorName` (`WidgetComponent.GetWidget` (`self.Widget`))))
  (`TextBlock.SetText` (`/Game/Widgets/WBP_ActorName.actorName` _aswbp_actor_name) (`self.Name`)))

(fn `UpdateCharacter`
  (bind _outrownames (`DataTableFunctionLibrary.GetDataTableRowNames` "/Game/Systems/Characters/Datatable/DT_Dialog.DT_Dialog"))
  (for _array_element _outrownames
    (bind _returnvalue (`|GetDataTableRow` "/Game/Systems/Characters/Datatable/DT_Dialog.DT_Dialog" _array_element)
      (:`then`
        (bind (_dialogtextarray _character _event) (break `/Game/Systems/Characters/Structure/S_Dialog` _returnvalue))
        (bind _returnvalue_2 (`GameplayStatics.GetActorOfClass` _character))
        (if (and (== _returnvalue_2 self) (`|EnumEquality` _event (`self.Event`)))
          (set `self.dialogTextArray` _dialogtextarray))))))

(fn `UserConstructionScript`)