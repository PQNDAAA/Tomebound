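; BP_Character is a talkable character actor with a name label and a click-to-open dialog.
; Overlapping its Box enables the actor's input and opens a gate; leaving reverses both.
; A left click whose cursor trace hits a "CharacterActor"-tagged component disables pawn input and shows WBP_CharacterDialog with the character's text array.
; A stored widget reference blocks duplicate dialogs until ResetDialogBox clears it.
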(event `Key|LeftMouseButton`
  (params (Key :type "Key Structure"))
  (bind (_bblockinghit _binitialoverlap _time _distance _location _impactpoint _normal _impactnormal _physmat _hitactor _hitcomponent) (`GameplayStatics.BreakHitResult` (`PlayerController.GetHitResultUnderCursorByChannel` (`GameplayStatics.GetPlayerController` 0) "TraceTypeQuery1" true)))
  (:`Pressed`
    (`/Engine/EditorBlueprintResources/StandardMacros.IsValid` _hitcomponent
      (:`Is Valid`
        (if (and (`ActorComponent.ComponentHasTag` _hitcomponent "CharacterActor") (not (`KismetSystemLibrary.IsValid` (`self.dialogBox_Reference`))))
          (`/Engine/EditorBlueprintResources/StandardMacros.Gate` true :!label _label
            (:`Exit`
              (`self.DisableInput` (`GameplayStatics.GetPlayerPawn` 0) (`GameplayStatics.GetPlayerController` 0))
              (bind _returnvalue (`|CreateWidget` "/Game/Widgets/WBP_CharacterDialog.WBP_CharacterDialog_C" null self (`self.dialogTextArray`)))
              (bind _output_get (set `self.dialogBox_Reference` _returnvalue))
              (`UserWidget.AddToViewport` _output_get 0))))))))

(event `self.Box.OnComponentBeginOverlap`
  (params (OverlappedComponent :type "PrimitiveComponent Object Reference") (OtherActor :type "Actor Object Reference") (OtherComp :type "PrimitiveComponent Object Reference") (OtherBodyIndex :type Integer) (bFromSweep :type Boolean) (SweepResult :type "HitResult Structure (by ref)"))
  (`self.EnableInput` (`GameplayStatics.GetPlayerController` 0))
  (goto _label :!via `Open`))

(event `self.Box.OnComponentEndOverlap`
  (params (OverlappedComponent :type "PrimitiveComponent Object Reference") (OtherActor :type "Actor Object Reference") (OtherComp :type "PrimitiveComponent Object Reference") (OtherBodyIndex :type Integer))
  (`self.DisableInput` (`GameplayStatics.GetPlayerController` 0))
  (goto _label :!via `Close`))

(fn `ResetDialogBox`
  (set `self.dialogBox_Reference` null))

(fn `SetActorNameOnWidget`
  (bind _aswbp_actor_name (cast `/Game/Widgets/WBP_ActorName` (`WidgetComponent.GetWidget` (`self.Widget`))))
  (`TextBlock.SetText` (`/Game/Widgets/WBP_ActorName.actorName` _aswbp_actor_name) (`self.Name`)))

(fn `UserConstructionScript`)